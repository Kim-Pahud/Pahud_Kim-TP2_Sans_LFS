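; BP_Frigo is a fridge furniture actor that serves as a hiding spot for the player.
; Child-actor player zone events track presence and toggle the HideF key prompt, with exit also clearing the hidden flag.
; Interacting inside the zone flips the hidden flag and prompt, then swings the door open and shut with MoveComponentTo, without moving the player.
; Alien zone enter and exit events are bound but empty.
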(event Custom|On%20Player%20Enter
  (params (Object :type Actor%20Object%20Reference))
  (Variables|Default|SetIsPlayerIn? true)
  (CallFunction|Show/HideKey))

(event Custom|On%20Player%20Exit
  (params (Object :type Actor%20Object%20Reference))
  (Variables|Default|SetIsPlayerIn? false)
  (CallFunction|Show/HideKey)
  (Variables|Default|SetIsPlayerHiden? false))

(event Custom|On%20Alien%20Enter
  (params (Object :type Actor%20Object%20Reference)))

(event Custom|On%20Alien%20Exit
  (params (Object :type Actor%20Object%20Reference)))

(event Custom|Entrer/Sortir%20Frigo
  (if (Variables|Default|GetIsPlayerHiden?)
    (Variables|Default|SetIsPlayerHiden? false)
    (Rendering|SetVisibility (Variables|Default|GetHide%20%28F%29) true false)
    (else
      (Variables|Default|SetIsPlayerHiden? true)
      (Rendering|SetVisibility (Variables|Default|GetHide%20%28F%29) false false)))
  (Components|MoveComponentTo (Variables|Default|GetdoorFridge1) "3.000000,-1.666600,8.000000" "0.000000,110.000000,0.000000" false false 0.5 false)
  (Components|MoveComponentTo (Variables|Default|GetdoorFridge1) "3.000000,-1.666600,8.000000" "0.000000,0.000000,0.000000" false false 0.5 false))

(event Input|EnhancedActionEvents|EnhancedInputActionIA_Interact
  (params (ActionValue :type Boolean) (ElapsedSeconds :type Float%20%28double-precision%29) (TriggeredSeconds :type Float%20%28double-precision%29) (InputAction :type Input%20Action%20Object%20Reference :default "/Game/Game/Systeme/Character/CustomInputs/IA_Interact.IA_Interact"))
  (if (Variables|Default|GetIsPlayerIn?)
    (CallFunction|Entrer/SortirFrigo)))

(event EventBeginPlay
  (bind _asbp_enter_zone_player (Utilities|Casting|CastToBP_EnterZone_Player (Variables|/Script/Engine.ChildActorComponent|GetChildActor (Variables|Default|GetPlayerZone))))
  (bind _output_get (Variables|Default|SetAs%20BP%20Enter%20Zone%20Player _asbp_enter_zone_player))
  (EventDispatchers|BindEventtoOnPlayerEnter _output_get (EventDispatchers|CreateEvent :!event Custom|On%20Player%20Enter))
  (EventDispatchers|BindEventtoOnPlayerExit _output_get (EventDispatchers|CreateEvent :!event Custom|On%20Player%20Exit))
  (bind _asbp_enter_zone_alien (Utilities|Casting|CastToBP_EnterZone_Alien (Variables|/Script/Engine.ChildActorComponent|GetChildActor (Variables|Default|GetAlienZone))))
  (bind _output_get_2 (Variables|Default|SetAs%20BP%20Enter%20Zone%20Alien _asbp_enter_zone_alien))
  (EventDispatchers|BindEventtoOnAlienEnter _output_get_2 (EventDispatchers|CreateEvent :!event Custom|On%20Alien%20Enter))
  (EventDispatchers|BindEventtoOnAlienExit _output_get_2 (EventDispatchers|CreateEvent :!event Custom|On%20Alien%20Exit))
  (Rendering|SetVisibility (Variables|Default|GetHide%20%28F%29) false false)
  (Input|EnableInput (Game|GetPlayerController 0)))

(fn ConstructionScript)

(fn Show/HideKey
  (if (Variables|Default|GetIsKeyVisible?)
    (Rendering|SetVisibility (Variables|Default|GetHide%20%28F%29) false false)
    (Variables|Default|SetIsKeyVisible? false)
    (else
      (Rendering|SetVisibility (Variables|Default|GetHide%20%28F%29) true false)
      (Variables|Default|SetIsKeyVisible? true))))