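; BP_LavaBall is a lava ball moved by physics forces on its static mesh.
; Every Tick, a priority chain of boolean flags selects one constant world-axis force along X or Y, with a weaker push for go-back.
; The final +X branch repeats the IsBallGoX check from an earlier branch, so it never runs.
; The graph only reads these flags and never sets them.
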(event EventTick
  (params (DeltaSeconds :type Float%20%28single-precision%29))
  ;[0.15 0.15 0.15 0.5] Make LavaBall Move
  (if (Variables|Default|GetHasBallForce)
    (Physics|AddForce (Variables|Debug|GetStaticMeshComponent) "0.000000,-13000.000000,0.000000" "None" false)
    (elif (Variables|Default|GetIsBallGoBack)
      (Physics|AddForce (Variables|Debug|GetStaticMeshComponent) "0.000000,5500.000000,0.000000" "None" false)
      (elif (Variables|Default|GetIsBallGoX)
        (Physics|AddForce (Variables|Debug|GetStaticMeshComponent) "-13000.000000,0.000000,0.000000" "None" false)
        (elif (Variables|Default|GetIsBallGoFront)
          (Physics|AddForce (Variables|Debug|GetStaticMeshComponent) "0.000000,13000.000000,0.000000" "None" false)
          (elif (Variables|Default|GetIsBallGo-X)
            (Physics|AddForce (Variables|Debug|GetStaticMeshComponent) "13000.000000,0.000000,0.000000" "None" false)))))))

(fn ConstructionScript)