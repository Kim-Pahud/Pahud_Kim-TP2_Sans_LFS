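; BP_Door2 is a door that shows a "Press F" text prompt when the player is able to open it.
; On BeginPlay it binds to can/can't-open events from its BP_SpawnDoor2Zone child actor and caches the game mode.
; The prompt and IsDoorOpenable flag turn on only if the door is closed and the game mode's fuse box is activated.
; Tick hides the prompt once IsDoorOpen is true; the opening itself happens outside this graph.
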(event Custom|Player%20Cant%20Open
  ;[0.15 0.15 0.15 0.5] Visibility (Press f) Door2
  (Rendering|SetVisibility (Variables|Default|GetTextRender) false false)
  (Variables|Default|SetIsDoorOpenable false))

(event Custom|Player%20Can%20Open
  ;[0.15 0.15 0.15 0.5] Visibility (Press f) Door2
  (if (not (Variables|Default|GetIsDoorOpen))
    (if (Variables|/Game/ThirdPerson/Blueprints/BP_ThirdPersonGameMode.BP_ThirdPersonGameMode_C|GetIsFuseBoxActivated (stale EventBeginPlay _asbp_third_person_game_mode))
      (Rendering|SetVisibility (Variables|Default|GetTextRender) true false)
      (Variables|Default|SetIsDoorOpenable true))))

(event EventBeginPlay
  ;[0.15 0.15 0.15 0.5] Visibility (Press f) Door2
  (bind _asbp_spawn_door_2zone (Utilities|Casting|CastToBP_SpawnDoor2Zone (Variables|/Script/Engine.ChildActorComponent|GetChildActor (Variables|Default|GetBP_SpawnDoor2Zone))))
  (EventDispatchers|BindEventtoPlayerCanOpenDoor2 _asbp_spawn_door_2zone (delegate Custom|Player%20Can%20Open))
  (EventDispatchers|BindEventtoPlayerCantOpenDoor2 _asbp_spawn_door_2zone (delegate Custom|Player%20Cant%20Open))
  (bind _asbp_third_person_game_mode (Utilities|Casting|CastToBP_ThirdPersonGameMode (Game|GetGameMode))))

(event EventTick
  (params (DeltaSeconds :type Float%20%28single-precision%29))
  ;[0.15 0.15 0.15 0.5] Visibility (Press f) Door2
  (if (not (Variables|Default|GetIsTextHidden))
    (if (Variables|Default|GetIsDoorOpen)
      (Rendering|SetVisibility (Variables|Default|GetTextRender) false false)
      (Variables|Default|SetIsTextHidden true))))

(fn ConstructionScript)