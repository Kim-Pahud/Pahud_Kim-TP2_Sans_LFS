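; BP_BlinkLight is a status light that reflects whether the engine has fuel.
; On BeginPlay it caches the BP_ThirdPersonGameMode and the BP_FuseBlinker_Blueprint held in its Blinker child actor component.
; Each Tick it polls EngineHasFuel on the game mode: with fuel it calls ColorChanger with its RGBA variables, otherwise it calls Blinker with the frame delta, max intensity and speed multiplier.
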(event EventBeginPlay
  (bind _asbp_third_person_game_mode (Utilities|Casting|CastToBP_ThirdPersonGameMode (Game|GetGameMode)))
  (bind _output_get (Variables|Default|SetAs%20BP%20Third%20Person%20Game%20Mode _asbp_third_person_game_mode))
  (bind _asbp_fuse_blinker_blueprint (Utilities|Casting|CastToBP_FuseBlinker_Blueprint (Variables|/Script/Engine.ChildActorComponent|GetChildActor (Variables|Default|GetBlinker))))
  (bind _output_get_2 (Variables|Default|SetAs%20BP%20Fuse%20Blinker%20Blueprint _asbp_fuse_blinker_blueprint)))

(event EventTick
  (params (DeltaSeconds :type Float%20%28single-precision%29))
  (if (Variables|/Game/ThirdPerson/Blueprints/BP_ThirdPersonGameMode.BP_ThirdPersonGameMode_C|GetEngineHasFuel (stale EventBeginPlay _output_get))
    (Default|ColorChanger (stale EventBeginPlay _output_get_2) (Variables|Default|GetR) (Variables|Default|GetG) (Variables|Default|GetB) (Variables|Default|GetA))
    (else
      (Default|Blinker (stale EventBeginPlay _output_get_2) DeltaSeconds (Variables|Default|GetMaxIntensity) (Variables|Default|GetDeltaMult)))))

(fn ConstructionScript)