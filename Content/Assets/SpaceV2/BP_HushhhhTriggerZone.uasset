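; BP_HushhhhTriggerZone is a trigger actor that starts and stops the player's "Ushhh" sound, gated by the game mode's drone arrival state.
; It caches BP_ThirdPersonGameMode on BeginPlay.
; A Player-tagged actor entering calls CallPlayerUshhh only if the drone has not arrived.
; Exiting calls CallPlayerStopUshhh only if the drone has arrived, so leaving before then does not trigger the stop.
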(event EventBeginPlay
  (bind _asbp_third_person_game_mode (Utilities|Casting|CastToBP_ThirdPersonGameMode (Game|GetGameMode)))
  (bind _output_get (Variables|Default|SetAs%20BP%20Third%20Person%20Game%20Mode _asbp_third_person_game_mode)))

(event Collision|EventActorBeginOverlap
  (params (OtherActor :type Actor%20Object%20Reference))
  ;[0.15 0.15 0.15 0.5] Trigger For Ushhh Sound
  (if (Actor|ActorHasTag OtherActor "Player")
    (if (not (Variables|/Game/ThirdPerson/Blueprints/BP_ThirdPersonGameMode.BP_ThirdPersonGameMode_C|GetIsDroneArrived (stale EventBeginPlay _output_get)))
      (Default|CallPlayerUshhh))))

(event Collision|EventActorEndOverlap
  (params (OtherActor :type Actor%20Object%20Reference))
  ;[0.15 0.15 0.15 0.5] Trigger To Stop Ushhh Sound
  (if (Actor|ActorHasTag OtherActor "Player")
    (if (Variables|/Game/ThirdPerson/Blueprints/BP_ThirdPersonGameMode.BP_ThirdPersonGameMode_C|GetIsDroneArrived (stale EventBeginPlay _output_get))
      (Default|CallPlayerStopUshhh))))

(fn ConstructionScript)