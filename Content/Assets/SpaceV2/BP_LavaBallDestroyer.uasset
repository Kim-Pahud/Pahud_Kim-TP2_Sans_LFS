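; BP_LavaBallDestroyer is an overlap trigger that destroys actors tagged LavaBall and restores the lights.
; On overlap it sets LightCheck on the third-person game mode, stops an audio component and destroys the ball.
; It then loops over every BP_SpawnLight to switch it on, with delayed voice-over lines chained inside that loop.
; The final go-back-to-pod line plays only if the game mode's GameFinished flag is unset.
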(event Collision|EventActorBeginOverlap
  (params (OtherActor :type Actor%20Object%20Reference))
  ;[0.15 0.15 0.15 0.5] Destroy LavaBall, Stop It's Sound And Open Lights
  (if (Actor|ActorHasTag OtherActor "LavaBall")
    (Variables|/Game/ThirdPerson/Blueprints/BP_ThirdPersonGameMode.BP_ThirdPersonGameMode_C|SetLightCheck (stale EventBeginPlay _output_get) true)
    (Utilities|IsValid OtherActor
      (:Is%20Valid
        (Audio|Components|Audio|Stop (Actor|GetComponentbyClass "/Script/Engine.AudioComponent"))
        (Actor|DestroyActor OtherActor)
        (bind _outactors (Actor|GetAllActorsOfClass "/Game/Assets/SpaceV2/BP_SpawnLight.BP_SpawnLight_C"))
        (for _array_element _outactors
          (Default|Lighton _array_element)
          (Audio|Components|Audio|Play (Variables|Default|GetVO_light-sys-on) 0.0)
          (Utilities|FlowControl|Delay 4.0)
          (Audio|Components|Audio|Play (Variables|Default|GetVO_Company_thx_you) 0.0)
          (Utilities|FlowControl|Delay 25.0)
          (if (not (Variables|/Game/ThirdPerson/Blueprints/BP_ThirdPersonGameMode.BP_ThirdPersonGameMode_C|GetGameFinished (stale EventBeginPlay _output_get)))
            (Audio|Components|Audio|Play (Variables|Default|GetVO_go-back-pod) 0.0)))))))

(event EventBeginPlay
  ;[0.15 0.15 0.15 0.5] Destroy LavaBall, Stop It's Sound And Open Lights
  (bind _asbp_third_person_game_mode (Utilities|Casting|CastToBP_ThirdPersonGameMode (Game|GetGameMode)))
  (bind _output_get (Variables|Default|SetAs%20BP%20Third%20Person%20Game%20Mode _asbp_third_person_game_mode)))

(fn ConstructionScript)