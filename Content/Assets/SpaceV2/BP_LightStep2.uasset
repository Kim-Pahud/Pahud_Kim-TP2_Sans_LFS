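; BP_LightStep2 manages the step 2 spotlights, driven by the pile and drone flags in BP_ThirdPersonGameMode.
; While the pile is in the drone, Tick shows both lights once after the LightOpeningDelay timeline, playing the Off sounds.
; A 0.2-second Delay re-rolls against LightRate to flicker the parent spotlight's intensity with a blink sound.
; Once the drone arrives, Tick hides both lights and plays the On sounds every frame.
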(event EventTick
  (params (DeltaSeconds :type Float%20%28single-precision%29))
  ;[0.15 0.15 0.15 0.5] Manage Light For Step2
  (if (Variables|/Game/ThirdPerson/Blueprints/BP_ThirdPersonGameMode.BP_ThirdPersonGameMode_C|GetIsPileInDrone (stale EventBeginPlay _asbp_third_person_game_mode))
    (if (Variables|/Game/ThirdPerson/Blueprints/BP_ThirdPersonGameMode.BP_ThirdPersonGameMode_C|GetIsDroneArrived (stale EventBeginPlay _asbp_third_person_game_mode))
      (Rendering|SetVisibility (Variables|Default|GetSpotLightComponent) false false)
      (Rendering|SetVisibility (Components|GetChildComponent (Variables|Default|GetSpotLight) 0) false false)
      ;[0.15 0.15 0.15 0.5] Play Light Sounds
      (Audio|Components|Audio|Play (Variables|Default|GetOn) 0.0)
      (Audio|Components|Audio|Play (Variables|Default|GetOn1) 0.0)
      (else
        (Utilities|FlowControl|Sequence
          (:then_0
            (Utilities|FlowControl|DoOnce false
              (:Completed
                (Timeline|Light%20OpeningDelay Play
                  (:Finished
                    (Rendering|SetVisibility (Variables|Default|GetSpotLightComponent) true false)
                    (Rendering|SetVisibility (Components|GetChildComponent (Variables|Default|GetSpotLight) 0) true false)
                    (Audio|Components|Audio|Play (Variables|Default|GetOff) 0.0)
                    (Audio|Components|Audio|Play (Variables|Default|GetOff1) 0.0))))))
          (:then_1
            ;[0.15 0.15 0.15 0.5] Make The Parent Spot Light Blink
            (Utilities|FlowControl|Delay 0.2)
            (if (> (Math|Random|RandomFloatinRange 0.0 1.0) (Variables|Default|GetLightRate))
              (Rendering|Components|Light|SetIntensity (Variables|Default|GetSpotLightComponent) 1e+04)
              (Audio|Components|Audio|Play (Variables|Default|GetBlink) 0.0)
              (else
                (Rendering|Components|Light|SetIntensity (Variables|Default|GetSpotLightComponent) 5e+04)))))))))

(event EventBeginPlay
  ;[0.15 0.15 0.15 0.5] Manage Light For Step2
  (bind _asbp_third_person_game_mode (Utilities|Casting|CastToBP_ThirdPersonGameMode (Game|GetGameMode))))

(fn ConstructionScript)