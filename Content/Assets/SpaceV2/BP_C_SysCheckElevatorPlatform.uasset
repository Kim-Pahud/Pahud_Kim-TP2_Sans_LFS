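; Elevator platform and pulley actor that animates when a ball drops into its pit, detected by a BP_MetBallZone child actor.
; On the zone's overlap event it lights five point lights, plays a chain sound and moves two cable components simultaneously over a fixed time.
; When the first cable finishes moving, it stops the sound, turns off the lights and sets PlateArrived on BP_ThirdPersonGameMode.
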(event Custom|MethBallInPit
  ;[0.15 0.15 0.15 0.5] Poulie And Elevator Animations
  (Rendering|SetVisibility (Variables|Default|GetPointLight1) true false)
  (Rendering|SetVisibility (Variables|Default|GetPointLight2) true false)
  (Rendering|SetVisibility (Variables|Default|GetPointLight3) true false)
  (Rendering|SetVisibility (Variables|Default|GetPointLight4) true false)
  (Rendering|SetVisibility (Variables|Default|GetPointLight5) true false)
  (Utilities|FlowControl|Sequence
    (:then_0
      (Components|MoveComponentTo (Variables|Default|Getcable8) "95.000000,95.000000,510.000000" "-90.000000,0.000000,0.000000" false false 2.5 false)
      (Audio|Components|Audio|Stop (Variables|Default|GetS_ChainSound))
      (Rendering|SetVisibility (Variables|Default|GetPointLight1) false false)
      (Rendering|SetVisibility (Variables|Default|GetPointLight2) false false)
      (Rendering|SetVisibility (Variables|Default|GetPointLight3) false false)
      (Rendering|SetVisibility (Variables|Default|GetPointLight4) false false)
      (Rendering|SetVisibility (Variables|Default|GetPointLight5) false false)
      (Variables|/Game/ThirdPerson/Blueprints/BP_ThirdPersonGameMode.BP_ThirdPersonGameMode_C|SetPlateArrived (stale EventBeginPlay _output_get) true))
    (:then_1
      (Audio|Components|Audio|Play (Variables|Default|GetS_ChainSound) 0.0)
      (Components|MoveComponentTo (Variables|Default|Getcable9) "695.000000,95.000000,12.000000" "-90.000000,0.000000,0.000000" false false 2.5 false))))

(event EventBeginPlay
  ;[0.15 0.15 0.15 0.5] Poulie And Elevator Animations
  (bind _asbp_met_ball_zone (Utilities|Casting|CastToBP_MetBallZone (Variables|/Script/Engine.ChildActorComponent|GetChildActor (Variables|Default|GetMetBallZone))))
  (EventDispatchers|BindEventtoOnMetBallOverlapin _asbp_met_ball_zone (delegate Custom|MethBallInPit))
  (bind _asbp_third_person_game_mode (Utilities|Casting|CastToBP_ThirdPersonGameMode (Game|GetGameMode)))
  (bind _output_get (Variables|Default|SetAs%20BP%20Third%20Person%20Game%20Mode _asbp_third_person_game_mode)))

(fn ConstructionScript)