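; BP_LightStep1 is a light fixture with three spot lights that react to fuse box and drone battery ("pile") state from BP_ThirdPersonGameMode.
; Tick polls both flags once the fuse box is activated, using DoOnce gates to switch lights and play sounds.
; Without the pile in the drone, lights appear after a short delay and the main spot flickers randomly between two intensities against LightRate.
; With it inserted, all three lights are hidden.
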(event EventTick
  (params (DeltaSeconds :type Float%20%28single-precision%29))
  ;[0.15 0.15 0.15 0.5] Set When Lights Are Visible
  (if (Variables|/Game/ThirdPerson/Blueprints/BP_ThirdPersonGameMode.BP_ThirdPersonGameMode_C|GetIsFuseBoxActivated (stale EventBeginPlay _output_get))
    (if (Variables|/Game/ThirdPerson/Blueprints/BP_ThirdPersonGameMode.BP_ThirdPersonGameMode_C|GetIsPileInDrone (stale EventBeginPlay _output_get))
      (Utilities|FlowControl|DoOnce false
        (:Completed
          (Rendering|SetVisibility (Variables|Default|GetSpotLightComponent) false false)
          (Rendering|SetVisibility (Components|GetChildComponent (Variables|Default|GetBlinkSpotLight1) 0) false false)
          (Rendering|SetVisibility (Components|GetChildComponent (Variables|Default|GetBlinkSpotLight) 0) false false)
          ;[0.15 0.15 0.15 0.5] Play Opening And Closing Light Sound
          (Audio|Components|Audio|Play (Variables|Default|GetAudio) 0.0)
          (Audio|Components|Audio|Play (Variables|Default|GetAudio3) 0.0)
          (Audio|Components|Audio|Play (Variables|Default|GetAudio5) 0.0)))
      (else
        (Utilities|FlowControl|Sequence
          (:then_0
            (Utilities|FlowControl|DoOnce false
              (:Completed
                (Utilities|FlowControl|Delay 0.28)
                (Rendering|SetVisibility (Variables|Default|GetSpotLightComponent) true false)
                (Rendering|SetVisibility (Components|GetChildComponent (Variables|Default|GetBlinkSpotLight1) 0) true false)
                (Rendering|SetVisibility (Components|GetChildComponent (Variables|Default|GetBlinkSpotLight) 0) true false)
                (Audio|Components|Audio|Play (Variables|Default|GetAudio1) 0.0)
                (Audio|Components|Audio|Play (Variables|Default|GetAudio) 0.0)
                (Audio|Components|Audio|Play (Variables|Default|GetAudio4) 0.0))))
          (:then_1
            ;[0.15 0.15 0.15 0.5] Make The Parent Spot Light Blink
            (Utilities|FlowControl|Delay 0.2)
            (if (> (Math|Random|RandomFloatinRange 0.0 1.0) (Variables|Default|GetLightRate))
              (Rendering|Components|Light|SetIntensity (Variables|Default|GetSpotLightComponent) 1e+04)
              (Audio|Components|Audio|Play (Variables|Default|GetS_BlinkSpotLight) 0.0)
              (else
                (Rendering|Components|Light|SetIntensity (Variables|Default|GetSpotLightComponent) 5e+04)))))))))

(event EventBeginPlay
  ;[0.15 0.15 0.15 0.5] Set When Lights Are Visible
  (bind _asbp_third_person_game_mode (Utilities|Casting|CastToBP_ThirdPersonGameMode (Game|GetGameMode)))
  (bind _output_get (Variables|Default|SetAs%20BP%20Third%20Person%20Game%20Mode _asbp_third_person_game_mode)))

(fn ConstructionScript)