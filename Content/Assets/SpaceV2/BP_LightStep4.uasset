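; BP_LightStep4 manages the spotlight for the domino step of a lava ball sequence.
; On BeginPlay it casts the child actors of DominoBallZone and LavaBall2Starter to their zone Blueprints and binds to their events.
; A lava ball entering the domino zone turns the spotlight on.
; A ball passing the LavaBall2 starter zone turns it off and plays VoiceLine12.
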(event Custom|LavaBallPassed
  ;[0.15 0.15 0.15 0.5] Light Management for Dominos
  (Rendering|SetVisibility (Variables|Default|GetSpotLightComponent) false false)
  (Audio|Components|Audio|Play (Variables|Default|GetVoiceLine12) 0.0))

(event Custom|LavaBallEnter
  ;[0.15 0.15 0.15 0.5] Light Management for Dominos
  (Rendering|SetVisibility (Variables|Default|GetSpotLightComponent) true false))

(event EventBeginPlay
  ;[0.15 0.15 0.15 0.5] Light Management for Dominos
  (bind _asbp_lava_ball_2starter_zone (Utilities|Casting|CastToBP_LavaBall2StarterZone (Variables|/Script/Engine.ChildActorComponent|GetChildActor (Variables|Default|GetLavaBall2Starter))))
  (EventDispatchers|BindEventtoLavaBallPassed _asbp_lava_ball_2starter_zone (delegate Custom|LavaBallPassed))
  (bind _asbp_domino_ball_zone (Utilities|Casting|CastToBP_DominoBallZone (Variables|/Script/Engine.ChildActorComponent|GetChildActor (Variables|Default|GetDomino%20Ball%20Zone))))
  (EventDispatchers|BindEventtoLavaBallEnter _asbp_domino_ball_zone (delegate Custom|LavaBallEnter)))

(fn ConstructionScript)