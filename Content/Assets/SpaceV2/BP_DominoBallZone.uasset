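; BP_DominoBallZone is a trigger volume for the lava ball, identified by its LavaBall tag.
; When a lava ball enters, it turns off the ball's force, flags it to go back and calls LavaBallEnter, noted as turning on lights.
; When the ball leaves, it clears the constraint mode on the ball's mesh so it moves freely.
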(event Collision|EventActorBeginOverlap
  (params (OtherActor :type Actor%20Object%20Reference))
  ;[0.15 0.15 0.15 0.5] Turn Off Ball Force And On Lights
  (if (Actor|ActorHasTag OtherActor "LavaBall")
    (bind _asbp_lava_ball (Utilities|Casting|CastToBP_LavaBall OtherActor))
    (Variables|/Game/Assets/SpaceV2/BP_LavaBall.BP_LavaBall_C|SetHasBallForce _asbp_lava_ball false)
    (Variables|/Game/Assets/SpaceV2/BP_LavaBall.BP_LavaBall_C|SetIsBallGoBack _asbp_lava_ball true)
    (Default|CallLavaBallEnter)))

(event Collision|EventActorEndOverlap
  (params (OtherActor :type Actor%20Object%20Reference))
  ;[0.15 0.15 0.15 0.5] Allow LavaBall To Be Free
  (if (Actor|ActorHasTag OtherActor "LavaBall")
    (bind _asbp_lava_ball (Utilities|Casting|CastToBP_LavaBall OtherActor))
    (Class|PrimitiveComponent|SetConstraintMode (Variables|/Script/Engine.StaticMeshActor|GetStaticMeshComponent _asbp_lava_ball) "None")))

(fn ConstructionScript)