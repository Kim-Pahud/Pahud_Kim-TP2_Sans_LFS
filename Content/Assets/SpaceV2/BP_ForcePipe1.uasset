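; BP_ForcePipe1 is a pipe actor that is visible and solid only while the game mode's IsPlayerOnPlate flag is true.
; BeginPlay caches BP_ThirdPersonGameMode, and Tick polls that flag.
; Two DoOnce gates that reset each other limit work to state changes, switching every static mesh component between visible with Block collision and hidden with Ignore collision.
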(event EventBeginPlay
  ;[0.15 0.15 0.15 0.5] Make all Pipe Diseapear and Get Rid Of Collisions
  ;[0.15 0.15 0.15 0.5] Reactivate Visibility And Collisions
  (bind _asbp_third_person_game_mode (Utilities|Casting|CastToBP_ThirdPersonGameMode (Game|GetGameMode)))
  (bind _output_get (Variables|Default|SetAs%20BP%20Third%20Person%20Game%20Mode _asbp_third_person_game_mode)))

(event EventTick
  (params (DeltaSeconds :type Float%20%28single-precision%29))
  (bind _returnvalue (Actor|GetComponentsByClass "/Script/Engine.StaticMeshComponent"))
  (bind _returnvalue_2 (Actor|GetComponentsByClass "/Script/Engine.StaticMeshComponent"))
  ;[0.15 0.15 0.15 0.5] Reactivate Visibility And Collisions
  (if (Variables|/Game/ThirdPerson/Blueprints/BP_ThirdPersonGameMode.BP_ThirdPersonGameMode_C|GetIsPlayerOnPlate (stale EventBeginPlay _output_get))
    (Utilities|FlowControl|DoOnce false :!label _label
      (:Completed
        (for _array_element _returnvalue
          (Collision|SetCollisionResponsetoAllChannels _array_element "ECR_Block"))
        (for _array_element_2 _returnvalue
          (Rendering|SetVisibility _array_element_2 true true)
          (goto _label_2 Reset))))
    (else
      ;[0.15 0.15 0.15 0.5] Make all Pipe Diseapear and Get Rid Of Collisions
      (Utilities|FlowControl|DoOnce false :!label _label_2
        (:Completed
          (for _array_element_3 _returnvalue_2
            (Collision|SetCollisionResponsetoAllChannels _array_element_3 "ECR_Ignore"))
          (for _array_element_4 _returnvalue_2
            (Rendering|SetVisibility _array_element_4 false true)
            (goto _label Reset)))))))

(fn ConstructionScript)