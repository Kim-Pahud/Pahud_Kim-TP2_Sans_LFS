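; BP_LightRack is a light rack that switches on its spotlights with sound when its check zone reports the light is on.
; Tick polls the child-actor BP_LightOnCheckZone's IsLightOn flag, but only while the game mode's LightCheck flag is false.
; A DoOnce then makes every spotlight component visible and plays six audio components, with no path to switch them back off.
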(event EventBeginPlay
  ;[0.15 0.15 0.15 0.5] Turn Light On In LightCheck And At The End
  (bind _asbp_third_person_game_mode (Utilities|Casting|CastToBP_ThirdPersonGameMode (Game|GetGameMode)))
  (bind _asbp_light_on_check_zone (Utilities|Casting|CastToBP_LightOnCheckZone (Variables|/Script/Engine.ChildActorComponent|GetChildActor (Variables|Default|GetLightOnCheckZone)))))

(event EventTick
  (params (DeltaSeconds :type Float%20%28single-precision%29))
  ;[0.15 0.15 0.15 0.5] Turn Light On In LightCheck And At The End
  (if (not (Variables|/Game/ThirdPerson/Blueprints/BP_ThirdPersonGameMode.BP_ThirdPersonGameMode_C|GetLightCheck (stale EventBeginPlay _asbp_third_person_game_mode)))
    (if (Variables|/Game/Assets/SpaceV2/BP_LightOnCheckZone.BP_LightOnCheckZone_C|GetIsLightOn (stale EventBeginPlay _asbp_light_on_check_zone))
      (Utilities|FlowControl|DoOnce false
        (:Completed
          (for _array_element (Actor|GetComponentsByClass "/Script/Engine.SpotLightComponent")
            (Rendering|SetVisibility _array_element true true))
          (Audio|Components|Audio|Play (Variables|Default|GetAudio1) 0.0)
          (Audio|Components|Audio|Play (Variables|Default|GetAudio2) 0.0)
          (Audio|Components|Audio|Play (Variables|Default|GetAudio3) 0.0)
          (Audio|Components|Audio|Play (Variables|Default|GetAudio4) 0.0)
          (Audio|Components|Audio|Play (Variables|Default|GetAudio) 0.0)
          (Audio|Components|Audio|Play (Variables|Default|GetAudio5) 0.0))))))

(fn ConstructionScript)