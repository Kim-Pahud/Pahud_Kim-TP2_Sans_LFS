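; BP_CrowBarSlot is a crowbar pickup slot that shows a Press F prompt and breaks its glass when taken.
; On BeginPlay it binds to the player in/out events of a child BP_FVisibilityZone, which toggle the prompt and CanTake flag.
; The prompt appears only while the game mode reports no crowbar held.
; TakeCrowbar, not called within this Blueprint, plays BreakWindow, reveals broken glass and hides prompt, platform and cable.
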(event Custom|PlayerCanTake
  ;[0.15 0.15 0.15 0.5] Make Press(F) Visible
  (if (not (Variables|/Game/ThirdPerson/Blueprints/BP_ThirdPersonGameMode.BP_ThirdPersonGameMode_C|GetPlayerHasCrowbar (stale EventBeginPlay _output_get)))
    (Rendering|SetVisibility (Variables|Default|GetPress%20%28F%29) true false)
    (Variables|Default|SetCanTake true)))

(event Custom|PlayerCantTake
  ;[0.15 0.15 0.15 0.5] Make Press(F) Visible
  (Rendering|SetVisibility (Variables|Default|GetPress%20%28F%29) false false)
  (Variables|Default|SetCanTake false))

(event EventBeginPlay
  ;[0.15 0.15 0.15 0.5] Make Press(F) Visible
  (bind _asbp_third_person_game_mode (Utilities|Casting|CastToBP_ThirdPersonGameMode (Game|GetGameMode)))
  (bind _output_get (Variables|Default|SetAs%20BP%20Third%20Person%20Game%20Mode _asbp_third_person_game_mode))
  (bind _asbp_fvisibility_zone (Utilities|Casting|CastToBP_FVisibilityZone (Variables|/Script/Engine.ChildActorComponent|GetChildActor (Variables|Default|GetCrowBarZone))))
  (bind _output_get_2 (Variables|Default|SetAs%20BP%20Crow%20Bar%20Zone _asbp_fvisibility_zone))
  (EventDispatchers|BindEventtoPlayerin _output_get_2 (delegate Custom|PlayerCanTake))
  (EventDispatchers|BindEventtoPlayerOut _output_get_2 (delegate Custom|PlayerCantTake)))

(fn ConstructionScript)

(fn TakeCrowbar
  ;[0.15 0.15 0.15 0.5] Make All Effects For Taking Crowbar
  (Audio|Components|Audio|Play (Variables|Default|GetBreakWindow) 0.0)
  (Rendering|SetVisibility (Variables|Default|GetPress%20%28F%29) false false)
  (Rendering|SetVisibility (Variables|Default|GetBrokenGlass1) true true)
  (Rendering|SetVisibility (Variables|Default|Getplatform_center) false false)
  (Rendering|SetVisibility (Variables|Default|Getcable) false false))