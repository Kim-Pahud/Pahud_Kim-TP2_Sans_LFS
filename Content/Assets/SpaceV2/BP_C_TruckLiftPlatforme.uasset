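; Truck lift platform Blueprint that animates when its child truck lift zone signals that a truck lift is ready.
; On BeginPlay it casts the TruckLiftZone child actor to BP_TruckLiftZone and binds to its ready event.
; The LiftBar timeline adds a vertical local offset to the high structure on every update, accumulating movement.
; Those updates also play the PlatformRotation timeline, which sets the small platform's relative roll.
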(event Custom|TruckLiftReady
  ;[0.15 0.15 0.15 0.5] Platform Lifting Animation
  (bind _liftbar (Timeline|LiftBar Play)
    (:Update
      (Transformation|AddLocalOffset (Variables|Default|Getstructure-high) (Math|Vector|MakeVector 0.0 0.0 _liftbar) false false)
      (bind _platformrotation (Timeline|PlatformRotation Play)
        (:Update
          (Transformation|SetRelativeRotation (Variables|Default|Getplatform_small) (Math|Rotator|MakeRotator _platformrotation 0.0 0.0) false false))))))

(event EventBeginPlay
  ;[0.15 0.15 0.15 0.5] Platform Lifting Animation
  (bind _asbp_truck_lift_zone (Utilities|Casting|CastToBP_TruckLiftZone (Variables|/Script/Engine.ChildActorComponent|GetChildActor (Variables|Default|GetTruckLiftZone))))
  (EventDispatchers|BindEventtoTruckLiftReady _asbp_truck_lift_zone (delegate Custom|TruckLiftReady)))

(fn ConstructionScript)