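; Stair spotlight actor that flickers once the game mode's second door is open, then goes dark for a jump scare.
; Tick uses a short Delay to throttle random rolls against LightRate, switching between a dimmed intensity with a sound and a brighter one.
; A BP_StairLightZone child actor's player-in event hides the light once and plays a second sound, which also ends the flicker through the visibility check.
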(event Custom|MakeJumpScare
  ;[0.15 0.15 0.15 0.5] Make JumpScare
  (Utilities|FlowControl|DoOnce false
    (:Completed
      (Rendering|SetVisibility (Variables|Default|GetSpotLight) false false)
      (Audio|Components|Audio|Play (Variables|Default|GetAudio1) 0.0))))

(event EventTick
  (params (DeltaSeconds :type Float%20%28single-precision%29))
  ;[0.15 0.15 0.15 0.5] Make StairLight Blink
  (if (Variables|/Game/ThirdPerson/Blueprints/BP_ThirdPersonGameMode.BP_ThirdPersonGameMode_C|GetIsDoor2Open (stale EventBeginPlay _output_get))
    (if (Rendering|IsVisible (Variables|Default|GetSpotLight))
      (Utilities|FlowControl|Delay 0.2)
      (if (> (Math|Random|RandomFloatinRange 0.0 1.0) (Variables|Default|GetLightRate))
        (Rendering|Components|Light|SetIntensity (Variables|Default|GetSpotLight) 1e+03)
        (Audio|Components|Audio|Play (Variables|Default|GetAudio) 0.0)
        (else
          (Rendering|Components|Light|SetIntensity (Variables|Default|GetSpotLight) 3e+03))))))

(event EventBeginPlay
  ;[0.15 0.15 0.15 0.5] Make JumpScare
  (bind _asbp_third_person_game_mode (Utilities|Casting|CastToBP_ThirdPersonGameMode (Game|GetGameMode)))
  (bind _output_get (Variables|Default|SetAs%20BP%20Third%20Person%20Game%20Mode _asbp_third_person_game_mode))
  (bind _asbp_stair_light_zone (Utilities|Casting|CastToBP_StairLightZone (Variables|/Script/Engine.ChildActorComponent|GetChildActor (Variables|Default|GetStairLightZone))))
  (EventDispatchers|BindEventtoPlayerin _asbp_stair_light_zone (delegate Custom|MakeJumpScare)))

(fn ConstructionScript)