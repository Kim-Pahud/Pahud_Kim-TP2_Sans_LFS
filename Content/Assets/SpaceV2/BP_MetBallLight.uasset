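; BP_MetBallLight is a light actor that switches its point light on while a met ball is inside its detection zone.
; On BeginPlay it casts its child actor to BP_MetBallLightZone and binds handlers to that zone's ball-in and ball-out events.
; The handlers show or hide the PointLight, propagating visibility to child components, so detection is left entirely to the zone.
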(event Custom|MetBallIn
  ;[0.15 0.15 0.15 0.5] Turn Light On When Met Ball Is Here
  (Rendering|SetVisibility (Variables|Default|GetPointLight) true true))

(event Custom|MetBallOut
  ;[0.15 0.15 0.15 0.5] Turn Light On When Met Ball Is Here
  (Rendering|SetVisibility (Variables|Default|GetPointLight) false true))

(event EventBeginPlay
  ;[0.15 0.15 0.15 0.5] Turn Light On When Met Ball Is Here
  (bind _asbp_met_ball_light_zone (Utilities|Casting|CastToBP_MetBallLightZone (Variables|/Script/Engine.ChildActorComponent|GetChildActor (Variables|Default|GetMetBallLightZone))))
  (EventDispatchers|BindEventtoMetBallin _asbp_met_ball_light_zone (delegate Custom|MetBallIn))
  (EventDispatchers|BindEventtoMetBallOut _asbp_met_ball_light_zone (delegate Custom|MetBallOut)))

(fn ConstructionScript)