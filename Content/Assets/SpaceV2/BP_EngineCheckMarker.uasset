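; BP_EngineCheckMarker is a trigger actor that completes the engine check when a LavaBall-tagged actor overlaps it.
; It caches the ThirdPerson game mode at BeginPlay and, on overlap, sets that game mode's EngineCheck flag.
; The same overlap starts the two Réacteur engine sounds at slightly different start times, stops the lava ball's audio component, then destroys the ball.
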(event Collision|EventActorBeginOverlap
  (params (OtherActor :type Actor%20Object%20Reference))
  ;[0.15 0.15 0.15 0.5] Set Engine Check Done
  (if (Actor|ActorHasTag OtherActor "LavaBall")
    (Variables|/Game/ThirdPerson/Blueprints/BP_ThirdPersonGameMode.BP_ThirdPersonGameMode_C|SetEngineCheck (stale EventBeginPlay _asbp_third_person_game_mode) true)
    ;[0.15 0.15 0.15 0.5] PlayEngineAudio
    (Audio|Components|Audio|Play (Variables|Default|GetRéacteur1) 0.1)
    (Audio|Components|Audio|Play (Variables|Default|GetRéacteur2) 0.0)
    ;[0.15 0.15 0.15 0.5] StopLavaBallSound
    (Audio|Components|Audio|Stop (Actor|GetComponentbyClass OtherActor "/Script/Engine.AudioComponent"))
    (Actor|DestroyActor OtherActor)))

(event EventBeginPlay
  ;[0.15 0.15 0.15 0.5] Set Engine Check Done
  (bind _asbp_third_person_game_mode (Utilities|Casting|CastToBP_ThirdPersonGameMode (Game|GetGameMode))))

(fn ConstructionScript)