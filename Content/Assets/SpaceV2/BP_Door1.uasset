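; Crowbar-gated door that shows a Press F prompt and plays a staged opening animation.
; A child BP_FVisibilityZone reports the player entering or leaving, toggling the prompt and CanOpen based on game mode crowbar and Door1Open flags.
; DoorOpeningAnimation, not triggered within this graph, hides the prompt, plays CrowbarDoorOpening and moves CorridorEnd in two eased steps separated by a delay.
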(event Custom|PlayerCanOpen
  ;[0.15 0.15 0.15 0.5] Make Press(F) Visible
  (if (Variables|/Game/ThirdPerson/Blueprints/BP_ThirdPersonGameMode.BP_ThirdPersonGameMode_C|GetPlayerHasCrowbar (stale EventBeginPlay _output_get))
    (if (not (Variables|/Game/ThirdPerson/Blueprints/BP_ThirdPersonGameMode.BP_ThirdPersonGameMode_C|GetDoor1Open (stale EventBeginPlay _output_get)))
      (Rendering|SetVisibility (Variables|Default|GetPress%20%28F%29) true false)
      (Variables|Default|SetCanOpen true))))

(event Custom|PlayerCantOpen
  ;[0.15 0.15 0.15 0.5] Make Press(F) Visible
  (Rendering|SetVisibility (Variables|Default|GetPress%20%28F%29) false false)
  (Variables|Default|SetCanOpen false))

(event Custom|DoorOpeningAnimation
  ;[0.15 0.15 0.15 0.5] Animation For the Door
  (Audio|Components|Audio|Play (Variables|Default|GetCrowbarDoorOpening) 0.0)
  (Rendering|SetVisibility (Variables|Default|GetPress%20%28F%29) false false)
  (Components|MoveComponentTo (Variables|Default|Getcorridor_end) "-7.000000,-5.000000,90.000000" "0.000000,180.000000,0.000000" true true 5.08 false)
  (Utilities|FlowControl|Delay 1.5)
  (Components|MoveComponentTo (Variables|Default|Getcorridor_end) "-7.000000,-5.000000,157.500000" "0.000000,180.000000,0.000000" true true 4.22 false))

(event EventBeginPlay
  ;[0.15 0.15 0.15 0.5] Make Press(F) Visible
  (bind _asbp_third_person_game_mode (Utilities|Casting|CastToBP_ThirdPersonGameMode (Game|GetGameMode)))
  (bind _output_get (Variables|Default|SetAs%20BP%20Third%20Person%20Game%20Mode _asbp_third_person_game_mode))
  (bind _asbp_fvisibility_zone (Utilities|Casting|CastToBP_FVisibilityZone (Variables|/Script/Engine.ChildActorComponent|GetChildActor (Variables|Default|GetIneractionRange))))
  (bind _output_get_2 (Variables|Default|SetAs%20BP%20FVisibility%20Zone _asbp_fvisibility_zone))
  (EventDispatchers|BindEventtoPlayerin _output_get_2 (delegate Custom|PlayerCanOpen))
  (EventDispatchers|BindEventtoPlayerOut _output_get_2 (delegate Custom|PlayerCantOpen)))

(fn ConstructionScript)