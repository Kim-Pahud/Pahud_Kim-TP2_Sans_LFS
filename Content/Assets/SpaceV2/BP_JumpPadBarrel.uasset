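; BP_JumpPadBarrel is a jump pad barrel that manages the lights signaling the jump pad arrival.
; On BeginPlay it casts its JumpZone child actor to BP_JumpPadBatrterieZone and binds LightOn to that zone's OnTriggerPileBoost event.
; LightOn shows four point lights when the event fires.
; A LightOff function hides the same lights but is not called within this Blueprint.
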(event Custom|LightOn
  ;[0.15 0.15 0.15 0.5] LightManagement for jumpPad Arrival
  (Rendering|SetVisibility (Variables|Default|GetPointLight) true false)
  (Rendering|SetVisibility (Variables|Default|GetPointLight1) true false)
  (Rendering|SetVisibility (Variables|Default|GetPointLight2) true false)
  (Rendering|SetVisibility (Variables|Default|GetPointLight3) true false))

(event EventBeginPlay
  ;[0.15 0.15 0.15 0.5] LightManagement for jumpPad Arrival
  (bind _asbp_jump_pad_batrterie_zone (Utilities|Casting|CastToBP_JumpPadBatrterieZone (Variables|/Script/Engine.ChildActorComponent|GetChildActor (Variables|Default|GetJumpZone))))
  (EventDispatchers|BindEventtoOnTriggerPileBoost _asbp_jump_pad_batrterie_zone (delegate Custom|LightOn)))

(fn ConstructionScript)

(fn LightOff
  (Rendering|SetVisibility (Variables|Default|GetPointLight) false false)
  (Rendering|SetVisibility (Variables|Default|GetPointLight1) false false)
  (Rendering|SetVisibility (Variables|Default|GetPointLight2) false false)
  (Rendering|SetVisibility (Variables|Default|GetPointLight3) false false))