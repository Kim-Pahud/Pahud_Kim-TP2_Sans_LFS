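; BP_LavaBallStarterZone is a trigger zone that sets lava balls rolling.
; An overlapping actor tagged LavaBall gets HasBallForce set on its BP_LavaBall and its AudioComponent started for the rolling sound.
; On BeginPlay it binds to the SoundStopper child BP_LavaBallEndSound's lava ball exit event, which stops the audio on the actor from the overlap event.
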(event Custom|StopRollingSound
  ;[0.15 0.15 0.15 0.5] Stop LavaBall Rolling Sound
  (Audio|Components|Audio|Stop (Actor|GetComponentbyClass (stale Collision|EventActorBeginOverlap OtherActor) "/Script/Engine.AudioComponent")))

(event EventBeginPlay
  ;[0.15 0.15 0.15 0.5] Stop LavaBall Rolling Sound
  (bind _asbp_lava_ball_end_sound (Utilities|Casting|CastToBP_LavaBallEndSound (Variables|/Script/Engine.ChildActorComponent|GetChildActor (Variables|Default|GetSoundStopper))))
  (EventDispatchers|BindEventtoLavaBallExit _asbp_lava_ball_end_sound (delegate Custom|StopRollingSound)))

(event Collision|EventActorBeginOverlap
  (params (OtherActor :type Actor%20Object%20Reference))
  ;[0.15 0.15 0.15 0.5] Make LavaBall Start
  (if (Actor|ActorHasTag OtherActor "LavaBall")
    (bind _asbp_lava_ball (Utilities|Casting|CastToBP_LavaBall OtherActor))
    (Variables|/Game/Assets/SpaceV2/BP_LavaBall.BP_LavaBall_C|SetHasBallForce _asbp_lava_ball true)
    ;[0.15 0.15 0.15 0.5] Play Lava Ball Rolling Sound
    (Audio|Components|Audio|Play (Actor|GetComponentbyClass OtherActor "/Script/Engine.AudioComponent") 0.0)))

(fn ConstructionScript)