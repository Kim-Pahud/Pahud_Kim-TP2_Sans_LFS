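; Level 2 door that slides open on player interaction when unlocked, or automatically for an alien.
; Enter and exit events toggle the interaction prompts, track whether the player can interact, and close the door on leaving.
; Opening and closing move the door mesh with MoveComponentTo and refresh front and back lights to reflect unlocked and open state.
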(event Custom|DoorClose
  ;[0.15 0.15 0.15 0.5] Door closing animation + update door light color
  (Variables|Default|SetIsOpen? false)
  (Default|LightColorChange (Variables|Default|GetBP_LightDoorBack) (Variables|Default|GetIsUnlocked?) (Variables|Default|GetIsOpen?))
  (Default|LightColorChange (Variables|Default|GetBP_LightDoorFront) (Variables|Default|GetIsUnlocked?) (Variables|Default|GetIsOpen?))
  (Components|MoveComponentTo (Variables|Default|GetMS_Props_corridor_end) "0, 0, 0" "0, 0, 0" false false 1.0 false))

(event Custom|DoorOpen
  ;[0.15 0.15 0.15 0.5] Door oppening animation + update door light color
  (if (Variables|Default|GetIsUnlocked?)
    (CallFunction|Show/HideInteractionKey (Variables|Default|GetIsOpen?))
    (Variables|Default|SetIsOpen? true)
    (Default|LightColorChange (Variables|Default|GetBP_LightDoorBack) (Variables|Default|GetIsUnlocked?) (Variables|Default|GetIsOpen?))
    (Default|LightColorChange (Variables|Default|GetBP_LightDoorFront) (Variables|Default|GetIsUnlocked?) (Variables|Default|GetIsOpen?))
    (Rendering|SetVisibility (Variables|Default|GetPress%28F%291) false false)
    (Components|MoveComponentTo (Variables|Default|GetMS_Props_corridor_end) "0.000000,0.000000,160.000000" "0, 0, 0" false false 1.0 false)))

(event Input|EnhancedActionEvents|EnhancedInputActionIA_Interact
  (params (ActionValue :type Boolean) (ElapsedSeconds :type Float%20%28double-precision%29) (TriggeredSeconds :type Float%20%28double-precision%29) (InputAction :type Input%20Action%20Object%20Reference :default "/Game/Game/Systeme/Character/CustomInputs/IA_Interact.IA_Interact"))
  ;[0.15 0.15 0.15 0.5] Play the door opening animation on player interaction
  (if (Variables|Default|GetCanOpen?)
    (CallFunction|DoorOpen)))

(event EventBeginPlay
  ;[0.15 0.15 0.15 0.5] Set default values of the door's lights and interaction sign
  (|CallParentFunction)
  (Rendering|SetVisibility (Variables|Default|GetPress%28F%29) false false)
  (Rendering|SetVisibility (Variables|Default|GetPress%28F%291) false false)
  (Default|LightColorChange (Variables|Default|GetBP_LightDoorBack) (Variables|Default|GetIsUnlocked?) false)
  (Default|LightColorChange (Variables|Default|GetBP_LightDoorFront) (Variables|Default|GetIsUnlocked?) false))

(event EventOnPlayerEnter
  (params (Object :type Actor%20Object%20Reference))
  ;[0.15 0.15 0.15 0.5] Set Interaction sign visibility and close the door if player leave
  (Variables|Default|SetCanOpen? true)
  (CallFunction|Show/HideInteractionKey (Variables|Default|GetIsOpen?))
  (Rendering|SetVisibility (Variables|Default|GetPress%28F%291) true false))

(event EventOnPlayerExit
  (params (Object :type Actor%20Object%20Reference))
  ;[0.15 0.15 0.15 0.5] Set Interaction sign visibility and close the door if player leave
  (Variables|Default|SetCanOpen? false)
  (CallFunction|Show/HideInteractionKey (Variables|Default|GetIsOpen?))
  (Rendering|SetVisibility (Variables|Default|GetPress%28F%291) false false)
  (if (Variables|Default|GetIsOpen?)
    (CallFunction|DoorClose)))

(event EventOnAlienEnter
  (params (Object :type Actor%20Object%20Reference))
  ;[0.15 0.15 0.15 0.5] Allow the alien to open / close door
  (CallFunction|Show/HideInteractionKey (Variables|Default|GetIsOpen?))
  (Rendering|SetVisibility (Variables|Default|GetPress%28F%291) true false)
  (CallFunction|DoorOpen))

(event EventOnAlienExit
  (params (Object :type Actor%20Object%20Reference))
  ;[0.15 0.15 0.15 0.5] Allow the alien to open / close door
  (CallFunction|Show/HideInteractionKey (Variables|Default|GetIsOpen?))
  (Rendering|SetVisibility (Variables|Default|GetPress%28F%291) false false)
  (CallFunction|DoorClose))

(fn ConstructionScript
  (|CallParentFunction))