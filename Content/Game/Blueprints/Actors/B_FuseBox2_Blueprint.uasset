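; Interactable fuse box actor that opens a cable-cutting puzzle widget when the player interacts inside its trigger zone.
; A child trigger zone toggles the Press F prompt and interaction; in Level_1 this also requires IsPlayerConnected.
; Cutting the right cable hides the prompt, stops it reappearing and calls GoodCableFromBox.
; Tick, throttled by DoOnce and Delay, then turns the child blinker from its configured color to red.
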(event Custom|GoodCable
  (Variables|Default|SetIsRightCableCut? true)
  (Rendering|SetVisibility (Variables|Default|GetPress%20%28F%29) false false)
  (Default|CallGoodCablefromBox))

(event Custom|OnPlayerEnter
  (params (Object :type Actor%20Object%20Reference))
  (if (Utilities|Enum|Equal(Enum) (Variables|Default|GetLevelName) "Level_1")
    (if (Variables|Default|GetIsPlayerConnected)
      (if (not (Variables|Default|GetIsRightCableCut?)) :!label _label
        (Rendering|SetVisibility (Variables|Default|GetPress%20%28F%29) true false)
        (Variables|Default|SetCanInteract? true)))
    (else
      (goto _label))))

(event Custom|OnPlayerExit
  (params (Object :type Actor%20Object%20Reference))
  (Rendering|SetVisibility (Variables|Default|GetPress%20%28F%29) false false)
  (Variables|Default|SetCanInteract? false))

(event Input|EnhancedActionEvents|EnhancedInputActionIA_Interact
  (params (ActionValue :type Boolean) (ElapsedSeconds :type Float%20%28double-precision%29) (TriggeredSeconds :type Float%20%28double-precision%29) (InputAction :type Input%20Action%20Object%20Reference :default "/Game/Game/Systeme/Character/CustomInputs/IA_Interact.IA_Interact"))
  (bind _widget (Variables|Default|GetWidget))
  (if (Variables|Default|GetCanInteract?)
    (Default|Activate/DesactivateCamInput (Variables|Default|GetAs%20BP%20Third%20Person%20Player%20Controller) _widget)
    (Variables|/Script/Engine.PlayerController|SetbShowMouseCursor (Game|GetPlayerController 0) true)
    (UserInterface|Viewport|AddtoViewport _widget 0)))

(event EventBeginPlay
  (bind _asbp_fuse_blinker_blueprint (Utilities|Casting|CastToBP_FuseBlinker_Blueprint (Variables|/Script/Engine.ChildActorComponent|GetChildActor (Variables|Default|GetCable_Box_Blinker))))
  (bind _output_get (Variables|Default|SetAs%20BP%20Fuse%20Blinker%20Blueprint _asbp_fuse_blinker_blueprint))
  (Default|ColorChanger _output_get (Variables|LightVar|GetR) (Variables|LightVar|GetG) (Variables|LightVar|GetB) (Variables|LightVar|GetA))
  (bind _asbp_third_person_player_controller (Utilities|Casting|CastToBP_ThirdPersonPlayerController (Game|GetPlayerController 0)))
  (Variables|Default|SetAs%20BP%20Third%20Person%20Player%20Controller _asbp_third_person_player_controller)
  (bind _asbp_enter_zone_player (Utilities|Casting|CastToBP_EnterZone_Player (Variables|/Script/Engine.ChildActorComponent|GetChildActor (Variables|Default|GetFuseTriggerZone))))
  (bind _output_get_2 (Variables|Default|SetAs%20BP%20Enter%20Zone%20Player _asbp_enter_zone_player))
  (EventDispatchers|BindEventtoOnPlayerEnter _output_get_2 (EventDispatchers|CreateEvent :!event Custom|OnPlayerEnter))
  (EventDispatchers|BindEventtoOnPlayerExit (Variables|Default|GetAs%20BP%20Enter%20Zone%20Player) (EventDispatchers|CreateEvent :!event Custom|OnPlayerExit))
  (bind _returnvalue (Game|GetCurrentLevelName true))
  (Variables|Default|SetLevelName _returnvalue)
  (bind _returnvalue_2 (UserInterface|CreateWidget "/Game/Game/UI/Actor_UI/WBP_CablePuzzle.WBP_CablePuzzle_C"))
  (bind _output_get_3 (Variables|Default|SetWidget _returnvalue_2))
  (EventDispatchers|BindEventtoGoodCable _output_get_3 (EventDispatchers|CreateEvent :!event Custom|GoodCable))
  (Rendering|SetVisibility (Variables|Default|GetPress%20%28F%29) false false)
  (Input|EnableInput (Game|GetPlayerController 0)))

(event EventTick
  (params (DeltaSeconds :type Float%20%28single-precision%29))
  (Utilities|FlowControl|DoOnce false :!label _label
    (:Completed
      (if (Variables|Default|GetIsRightCableCut?)
        (Default|ColorChanger (Variables|Default|GetAs%20BP%20Fuse%20Blinker%20Blueprint) 1.0 0.0 0.0 1.0))
      (Utilities|FlowControl|Delay 0.2)
      (goto _label Reset))))

(fn ConstructionScript)