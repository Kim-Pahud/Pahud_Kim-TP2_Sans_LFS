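; BP_Casier is a locker actor, apparently a hiding spot, with a door the player can open and close.
; Child-actor zones report player and alien overlaps through dispatchers, though the alien handlers are empty.
; Player enter and exit toggle the hide-key prompt and gate IA_Interact, which swings the door via MoveComponentTo.
; Exiting the zone clears IsOpen without moving the door.
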(event Custom|Entrer/Sorti%20Casier
  (if (Variables|Default|GetIsOpen?)
    (Components|MoveComponentTo (Variables|Default|GetPorte) "-92.634156,0.098604,-1.000001" "-0.000009,180.000000,180.000000" false false 0.5 false)
    (Variables|Default|SetIsOpen? false)
    (else
      (Components|MoveComponentTo (Variables|Default|GetPorte) "-92.634156,0.098604,-1.000001" "-89.000000,180.000000,180.000000" false false 0.5 false)
      (Variables|Default|SetIsOpen? true))))

(event Custom|On%20Player%20Enter
  (params (Object :type Actor%20Object%20Reference))
  (Variables|Default|SetIsPlayerIn? true)
  (CallFunction|Show/HideHideKey))

(event Custom|On%20Player%20Exit
  (params (Object :type Actor%20Object%20Reference))
  (Variables|Default|SetIsPlayerIn? false)
  (CallFunction|Show/HideHideKey)
  (Variables|Default|SetIsOpen? false))

(event Custom|On%20Alien%20Enter
  (params (Object :type Actor%20Object%20Reference)))

(event Custom|On%20Alien%20Exit
  (params (Object :type Actor%20Object%20Reference)))

(event Input|EnhancedActionEvents|EnhancedInputActionIA_Interact
  (params (ActionValue :type Boolean) (ElapsedSeconds :type Float%20%28double-precision%29) (TriggeredSeconds :type Float%20%28double-precision%29) (InputAction :type Input%20Action%20Object%20Reference :default "/Game/Game/Systeme/Character/CustomInputs/IA_Interact.IA_Interact"))
  (if (Variables|Default|GetIsPlayerIn?)
    (CallFunction|Entrer/SortiCasier)))

(event EventBeginPlay
  (bind _asbp_enter_zone_player (Utilities|Casting|CastToBP_EnterZone_Player (Variables|/Script/Engine.ChildActorComponent|GetChildActor (Variables|Default|GetPlayerZone))))
  (bind _output_get (Variables|Default|SetAs%20BP%20Enter%20Zone%20Player _asbp_enter_zone_player))
  (EventDispatchers|BindEventtoOnPlayerEnter _output_get (EventDispatchers|CreateEvent :!event Custom|On%20Player%20Enter))
  (EventDispatchers|BindEventtoOnPlayerExit _output_get (EventDispatchers|CreateEvent :!event Custom|On%20Player%20Exit))
  (bind _asbp_enter_zone_alien (Utilities|Casting|CastToBP_EnterZone_Alien (Variables|/Script/Engine.ChildActorComponent|GetChildActor (Variables|Default|GetAlienZone))))
  (bind _output_get_2 (Variables|Default|SetAs%20BP%20Enter%20Zone%20Alien _asbp_enter_zone_alien))
  (EventDispatchers|BindEventtoOnAlienEnter _output_get_2 (EventDispatchers|CreateEvent :!event Custom|On%20Alien%20Enter))
  (EventDispatchers|BindEventtoOnAlienExit _output_get_2 (EventDispatchers|CreateEvent :!event Custom|On%20Alien%20Exit))
  (Rendering|SetVisibility (Variables|Default|GetHide%20%28F%29) false false)
  (Input|EnableInput (Game|GetPlayerController 0)))

(fn ConstructionScript)

(fn Show/HideHideKey
  (if (Variables|Default|GetIsKeyVisible?)
    (Rendering|SetVisibility (Variables|Default|GetHide%20%28F%29) false false)
    (Variables|Default|SetIsKeyVisible? false)
    (else
      (Rendering|SetVisibility (Variables|Default|GetHide%20%28F%29) true false)
      (Variables|Default|SetIsKeyVisible? true))))