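; Connection desk actor that lets the player connect by interacting while in range, then broadcasts PlayerConnected.
; A child BP_EnterZone_Player reports enter and exit to set the range flag and swap the screen text; leaving unconnected also fires AngryAI as an easter egg.
; Tick blinks the text through a DoOnce reset after a Delay until connection.
; A DoOnce on IA_Interact resets on out-of-range presses, so connection happens only once.
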(event Custom|OnPlayerEnter
  (params (Object :type Actor%20Object%20Reference))
  ;[0.15 0.15 0.15 0.5] Set interaction range var and show easter egg text when player leave
  (if (not (Variables|Default|GetIsPlayerConnected?))
    (Variables|Default|SetIsPlayerIn? true)
    (CallFunction|ChangeScreenText)))

(event Custom|OnPlayerExit
  (params (Object :type Actor%20Object%20Reference))
  ;[0.15 0.15 0.15 0.5] Set interaction range var and show easter egg text when player leave
  (if (not (Variables|Default|GetIsPlayerConnected?))
    (Variables|Default|SetIsPlayerIn? false)
    (CallFunction|ChangeScreenText)))

(event Input|EnhancedActionEvents|EnhancedInputActionIA_Interact
  (params (ActionValue :type Boolean) (ElapsedSeconds :type Float%20%28double-precision%29) (TriggeredSeconds :type Float%20%28double-precision%29) (InputAction :type Input%20Action%20Object%20Reference :default "/Game/Game/Systeme/Character/CustomInputs/IA_Interact.IA_Interact"))
  (Utilities|FlowControl|DoOnce false :!label _label
    (:Completed
      (if (Variables|Default|GetIsPlayerIn?)
        (Variables|Default|SetIsPlayerConnected? true)
        (Rendering|SetVisibility (Variables|Default|GetConnect) false false)
        (Default|CallPlayerConnected)
        (else
          (goto _label Reset))))))

(event EventBeginPlay
  ;[0.15 0.15 0.15 0.5] Set all var, bind all event and inputs needed
  (bind _asbp_enter_zone_player (Utilities|Casting|CastToBP_EnterZone_Player (Variables|/Script/Engine.ChildActorComponent|GetChildActor (Variables|Default|GetInteraction%20Zone))))
  (EventDispatchers|BindEventtoOnPlayerEnter _asbp_enter_zone_player (EventDispatchers|CreateEvent :!event Custom|OnPlayerEnter))
  (EventDispatchers|BindEventtoOnPlayerExit _asbp_enter_zone_player (EventDispatchers|CreateEvent :!event Custom|OnPlayerExit))
  (Input|EnableInput (Game|GetPlayerController 0)))

(event EventTick
  (params (DeltaSeconds :type Float%20%28single-precision%29))
  ;[0.15 0.15 0.15 0.5] Make the text blink
  (Utilities|FlowControl|DoOnce false :!label _label
    (:Completed
      (if (Variables|Default|GetIsConnectVisible?)
        (Rendering|SetVisibility (Variables|Default|GetConnect) false false)
        (Variables|Default|SetIsConnectVisible? false)
        (else
          (Rendering|SetVisibility (Variables|Default|GetConnect) true false)
          (Variables|Default|SetIsConnectVisible? true)))
      (Utilities|FlowControl|Delay 1.0)
      (if (not (Variables|Default|GetIsPlayerConnected?))
        (goto _label Reset)))))

(fn ConstructionScript)

(fn ChangeScreenText
  (if (Variables|Default|GetIsPlayerIn?)
    (Rendering|Components|TextRender|SetText (Variables|Default|GetConnect) (Variables|Default|GetText2))
    (else
      (Rendering|Components|TextRender|SetText (Variables|Default|GetConnect) (Variables|Default|GetText1))
      (Default|CallAngryAI))))