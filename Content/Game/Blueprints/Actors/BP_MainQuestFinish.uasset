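; Interactable actor that marks the finish point of the main quest.
; Its child enter-zone actor reports player entry and exit, toggling the PressF prompt and an in-range flag.
; Pressing Interact while in range fires MainQuestDone, guarded by a DoOnce so it runs only once.
; A text render blinks continuously at one-second intervals through a self-resetting DoOnce and delays on Tick.
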(event Custom|On%20Player%20Enter
  (params (Object :type Actor%20Object%20Reference))
  (Variables|Default|SetIs%20Player%20In true)
  (Rendering|SetVisibility (Variables|Default|GetPress%20%28F%29) true false))

(event Custom|On%20Player%20Exit
  (params (Object :type Actor%20Object%20Reference))
  (Variables|Default|SetIs%20Player%20In false)
  (Rendering|SetVisibility (Variables|Default|GetPress%20%28F%29) false false))

(event Input|EnhancedActionEvents|EnhancedInputActionIA_Interact
  (params (ActionValue :type Boolean) (ElapsedSeconds :type Float%20%28double-precision%29) (TriggeredSeconds :type Float%20%28double-precision%29) (InputAction :type Input%20Action%20Object%20Reference :default "/Game/Game/Systeme/Character/CustomInputs/IA_Interact.IA_Interact"))
  (if (Variables|Default|GetIs%20Player%20In)
    (Utilities|FlowControl|DoOnce false
      (:Completed
        (Default|CallMainQuestDone)))))

(event EventBeginPlay
  (bind _asbp_enter_zone_player (Utilities|Casting|CastToBP_EnterZone_Player (Variables|/Script/Engine.ChildActorComponent|GetChildActor (Variables|Default|GetInteraction%20Zone))))
  (bind _output_get (Variables|Default|SetAs%20BP%20Enter%20Zone%20Player _asbp_enter_zone_player))
  (EventDispatchers|BindEventtoOnPlayerEnter _output_get (EventDispatchers|CreateEvent :!event Custom|On%20Player%20Enter))
  (EventDispatchers|BindEventtoOnPlayerExit _output_get (EventDispatchers|CreateEvent :!event Custom|On%20Player%20Exit))
  (Rendering|SetVisibility (Variables|Default|GetPress%20%28F%29) false false)
  (Input|EnableInput (Game|GetPlayerController 0)))

(event EventTick
  (params (DeltaSeconds :type Float%20%28single-precision%29))
  (Utilities|FlowControl|DoOnce false :!label _label
    (:Completed
      (Rendering|SetVisibility (Variables|Default|GetTextRender1) false false)
      (Utilities|FlowControl|Delay 1.0)
      (Rendering|SetVisibility (Variables|Default|GetTextRender1) true false)
      (Utilities|FlowControl|Delay 1.0)
      (goto _label Reset))))

(fn ConstructionScript)