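; Audio holder actor that owns the soundtrack (BO), background ambience and two camera sound components.
; BeginPlay plays an intro track, then after a fixed delay starts the main loop and ambience unless BoInterrupt is set.
; Chase events fade between main and chase music over two seconds, with the end event also setting BoInterrupt.
; Separate events play and stop each camera sound.
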(event Custom|Start%20BO_Chase
  ;[0.15 0.15 0.15 0.5] Make a transition from the main BO to the chasing BO
  (Utilities|FlowControl|Sequence
    (:then_0
      (Audio|Components|Audio|FadeOut (Variables|Default|GetBO_Boucle) 2.0 0.0 "Linear" :!class /Script/Engine.AudioComponent)
      (Audio|Components|Audio|FadeOut (Variables|Default|GetBO_Start) 2.0 0.0 "Linear" :!class /Script/Engine.AudioComponent)
      (Utilities|FlowControl|Delay 2.0)
      (Audio|Components|Audio|Stop (Variables|Default|GetBO_Boucle))
      (Audio|Components|Audio|Stop (Variables|Default|GetBO_Start)))
    (:then_1
      (Audio|Components|Audio|FadeIn (Variables|Default|GetBO_Chase) 2.0 1.0 0.0 "Linear" :!class /Script/Engine.AudioComponent))))

(event Custom|End%20BO_Chase
  ;[0.15 0.15 0.15 0.5] Make a transition from chasing BO to the main BO
  (Utilities|FlowControl|Sequence
    (:then_0
      (Audio|Components|Audio|FadeOut (Variables|Default|GetBO_Chase) 2.0 0.0 "Linear" :!class /Script/Engine.AudioComponent)
      (Utilities|FlowControl|Delay 2.0)
      (Audio|Components|Audio|Stop (Variables|Default|GetBO_Chase))
      (Variables|Default|SetBo%20Interrupt true))
    (:then_1
      (Audio|Components|Audio|Play (Variables|Default|GetBO_Boucle) 0.0)
      (Audio|Components|Audio|FadeIn (Variables|Default|GetBO_Boucle) 2.0 1.0 0.0 "Linear" :!class /Script/Engine.AudioComponent))))

(event Custom|Play%20Sound%20cam%201
  (Audio|Components|Audio|Play (Variables|Default|GetSound%20Cam%201) 0.0))

(event Custom|Play%20Sound%20Cam%202
  (Audio|Components|Audio|Play (Variables|Default|GetSound%20Cam%202) 0.0))

(event Custom|Stop%20cam%201
  (Audio|Components|Audio|Stop (Variables|Default|GetSound%20Cam%201)))

(event Custom|Stop%20cam%202
  (Audio|Components|Audio|Stop (Variables|Default|GetSound%20Cam%202)))

(event EventBeginPlay
  ;[0.15 0.15 0.15 0.5] Start the BO
  (Audio|Components|Audio|Play (Variables|Default|GetBO_Start) 0.0)
  (Utilities|FlowControl|Delay 23.293)
  (if (not (Variables|Default|GetBo%20Interrupt))
    (Audio|Components|Audio|Play (Variables|Default|GetBO_Boucle) 0.0)
    (Audio|Components|Audio|Play (Variables|Default|GetBKG%20Ambiance) 0.0)))

(fn ConstructionScript)