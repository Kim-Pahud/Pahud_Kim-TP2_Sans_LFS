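; Spawn door that the player opens through a code-entry widget, built on a parent door class with front and back status lights.
; When a connected player is in range, it enables interaction and updates the key prompt.
; Interacting shows WBP_DoorSpawnCode with a mouse cursor and toggles camera input through the player controller.
; DoorOpen slides the corridor-end mesh over time, while alien enter and exit events are left empty.
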(event Custom|DoorOpen
  (Components|MoveComponentTo (Variables|Default|GetMS_Props_corridor_end) "-7.000000,-5.000000,156.000000" "0.000000,180.000000,0.000000" true false 1.0 false))

(event Input|EnhancedActionEvents|EnhancedInputActionIA_Interact
  (params (ActionValue :type Boolean) (ElapsedSeconds :type Float%20%28double-precision%29) (TriggeredSeconds :type Float%20%28double-precision%29) (InputAction :type Input%20Action%20Object%20Reference :default "/Game/Game/Systeme/Character/CustomInputs/IA_Interact.IA_Interact"))
  (if (Variables|Default|GetCanOpen?)
    (bind _returnvalue (UserInterface|CreateWidget "/Game/Game/UI/Actor_UI/WBP_DoorSpawnCode.WBP_DoorSpawnCode_C"))
    (Default|Activate/DesactivateCamInput (Variables|Default|GetAs%20BP%20Third%20Person%20Player%20Controller) _returnvalue)
    (Variables|/Script/Engine.PlayerController|SetbShowMouseCursor (Game|GetPlayerController 0) true)
    (UserInterface|Viewport|AddtoViewport _returnvalue 0)))

(event EventOnPlayerExit
  (params (Object :type Actor%20Object%20Reference))
  (if (Variables|Default|GetIsPlayerConnected)
    (Variables|Default|SetCanOpen? false)
    (CallFunction|Show/HideInteractionKey (Variables|Default|GetIsOpen?))))

(event EventOnPlayerEnter
  (params (Object :type Actor%20Object%20Reference))
  (if (Variables|Default|GetIsPlayerConnected)
    (Variables|Default|SetCanOpen? true)
    (CallFunction|Show/HideInteractionKey (Variables|Default|GetIsOpen?))))

(event EventBeginPlay
  (|CallParentFunction)
  (bind _asbp_third_person_player_controller (Utilities|Casting|CastToBP_ThirdPersonPlayerController (Game|GetPlayerController 0)))
  (Variables|Default|SetAs%20BP%20Third%20Person%20Player%20Controller _asbp_third_person_player_controller)
  (Rendering|SetVisibility (Variables|Default|GetPress%28F%29) false false)
  (Default|LightColorChange (Variables|Default|GetBP_LightDoorBack) false false)
  (Default|LightColorChange (Variables|Default|GetBP_LightDoorFront) false false))

(event EventOnAlienEnter
  (params (Object :type Actor%20Object%20Reference)))

(event EventOnAlienExit
  (params (Object :type Actor%20Object%20Reference)))

(fn ConstructionScript
  (|CallParentFunction))