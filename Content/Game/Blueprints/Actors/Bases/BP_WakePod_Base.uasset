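; Base wake pod actor that opens in an emergency when the correct fuse box cable event fires.
; On BeginPlay it finds the B_FuseBox2_Blueprint actor, binds EmergencyOpen to its good-cable event and caches the level name.
; EmergencyOpen always calls CallOpen as a cue, and only in Level_1 also swaps a glass material on the Load component and animates it open with MoveComponentTo.
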(event Custom|EmergencyOpen
  ;[0.15 0.15 0.15 0.5] Open pod animation of level 1 + send a cue (usefull only for lvl2)
  (Default|CallOpen)
  (if (Utilities|Enum|Equal(Enum) (Variables|Default|GetLevelName) "Level_1")
    (Rendering|Material|SetMaterial (Variables|Default|Getload) 3 "/Game/Game/Materials/M_Vitre.M_Vitre")
    (Components|MoveComponentTo (Variables|Default|Getload) "28.644460,-3.667849,74.113936" "0.000000,-180.000004,280.000000" false false 3.0 false)))

(event EventBeginPlay
  ;[0.15 0.15 0.15 0.5] Set all event and var needed
  (bind _returnvalue (Actor|GetActorOfClass "/Game/Game/Blueprints/Actors/B_FuseBox2_Blueprint.B_FuseBox2_Blueprint_C"))
  (EventDispatchers|BindEventtoGoodCablefromBox _returnvalue (delegate Custom|EmergencyOpen))
  (bind _returnvalue_2 (Game|GetCurrentLevelName true))
  (Variables|Default|SetLevelName _returnvalue_2))

(fn ConstructionScript)