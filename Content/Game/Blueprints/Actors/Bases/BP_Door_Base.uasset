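; Base door actor that provides shared wiring for doors reacting to the player and aliens.
; On BeginPlay it binds enter/exit events from child-actor player and alien zones, caches front and back door lights, and enables input.
; Zone and interact handlers are empty here.
; A helper toggles the "Press F" prompt, always hiding it when the door is open.
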(event Custom|OnPlayerExit
  (params (Object :type Actor%20Object%20Reference)))

(event Custom|OnAlienExit
  (params (Object :type Actor%20Object%20Reference)))

(event Custom|OnAlienEnter
  (params (Object :type Actor%20Object%20Reference)))

(event Custom|OnPlayerEnter
  (params (Object :type Actor%20Object%20Reference)))

(event Input|EnhancedActionEvents|EnhancedInputActionIA_Interact
  (params (ActionValue :type Boolean) (ElapsedSeconds :type Float%20%28double-precision%29) (TriggeredSeconds :type Float%20%28double-precision%29) (InputAction :type Input%20Action%20Object%20Reference :default "/Game/Game/Systeme/Character/CustomInputs/IA_Interact.IA_Interact")))

(event EventBeginPlay
  (bind _asbp_enter_zone_alien (Utilities|Casting|CastToBP_EnterZone_Alien (Variables|/Script/Engine.ChildActorComponent|GetChildActor (Variables|Default|GetAlienZone))))
  (EventDispatchers|BindEventtoOnAlienEnter _asbp_enter_zone_alien (EventDispatchers|CreateEvent :!event Custom|OnAlienEnter))
  (EventDispatchers|BindEventtoOnAlienExit _asbp_enter_zone_alien (EventDispatchers|CreateEvent :!event Custom|OnAlienExit))
  (bind _asbp_enter_zone_player (Utilities|Casting|CastToBP_EnterZone_Player (Variables|/Script/Engine.ChildActorComponent|GetChildActor (Variables|Default|GetPlayerZone))))
  (EventDispatchers|BindEventtoOnPlayerEnter _asbp_enter_zone_player (EventDispatchers|CreateEvent :!event Custom|OnPlayerEnter))
  (EventDispatchers|BindEventtoOnPlayerExit _asbp_enter_zone_player (EventDispatchers|CreateEvent :!event Custom|OnPlayerExit))
  (bind _asbp_light_doors (Utilities|Casting|CastToBP_Light_Doors (Variables|/Script/Engine.ChildActorComponent|GetChildActor (Variables|Default|GetLightDoor_Front))))
  (Variables|Héritée|SetBP_LightDoorFront _asbp_light_doors)
  (bind _asbp_light_doors_2 (Utilities|Casting|CastToBP_Light_Doors (Variables|/Script/Engine.ChildActorComponent|GetChildActor (Variables|Default|GetLightDoor_Back))))
  (Variables|Héritée|SetBP_LightDoorBack _asbp_light_doors_2)
  (Input|EnableInput (Game|GetPlayerController 0)))

(fn ConstructionScript)

(fn Show/HideInteractionKey
  (params (IsOpen? :type Boolean))
  (if IsOpen?
    (Rendering|SetVisibility (Variables|Default|GetPress%28F%29) false false :!label _label)
    (Variables|Héritée|SetIsKeyVisible? false)
    (elif (Variables|Héritée|GetIsKeyVisible?)
      (goto _label)
      (else
        (Rendering|SetVisibility (Variables|Default|GetPress%28F%29) true false)
        (Variables|Héritée|SetIsKeyVisible? true)))))