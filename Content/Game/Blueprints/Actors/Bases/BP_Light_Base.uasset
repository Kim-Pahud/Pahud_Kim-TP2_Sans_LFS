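; BP_Light_Base is a base Blueprint for light actors with a point light that can be switched on and recolored for an angry AI state.
; LightOn makes the PointLight visible, with no matching off function.
; AngryAIColor alternates between dark red and warm white on each call, flipping IsAIAngry each time.
; The red is applied when the flag is true, which then resets it to false.
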(fn ConstructionScript)

(fn Lighton
  (Rendering|SetVisibility (Variables|Default|GetPointLight) true false))

(fn AngryAIColor
  (if (Variables|Default|GetIsAI_Angry?)
    (Rendering|Components|Light|SetLightColor (Variables|Default|GetPointLight) "(R=0.318547,G=0.000000,B=0.000094,A=1.000000)" true)
    (Variables|Default|SetIsAI_Angry? false)
    (else
      (Rendering|Components|Light|SetLightColor (Variables|Default|GetPointLight) "(R=1.000000,G=0.838799,B=0.617207,A=1.000000)" true)
      (Variables|Default|SetIsAI_Angry? true))))