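; BP_EmergencyLight is a blinking emergency light with an alarm sound, driven by state flags on BP_ThirdPersonGameMode.
; Once IsPileInDrone is set, Tick shows the point light and ramps its intensity up and down, toggled by IsLightMax.
; Each peak calls the LightMax dispatcher, whose bound event plays a 2D sound.
; IsDoor2Open takes priority, hiding the light and halting the blink.
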(event Custom|Sound
  ;[0.15 0.15 0.15 0.5] BlinkerTrackEmergency
  (Audio|PlaySound2D 0 0.03 1.0 0.0 0 0))

(event EventTick
  (params (DeltaSeconds :type Float%20%28single-precision%29))
  ;[0.15 0.15 0.15 0.5] BlinkerTrackEmergency
  (if (Variables|/Game/ThirdPerson/Blueprints/BP_ThirdPersonGameMode.BP_ThirdPersonGameMode_C|GetIsDoor2Open (stale EventBeginPlay _asbp_third_person_game_mode))
    (Rendering|SetVisibility (Variables|Default|GetPointLightComponent) false false)
    (elif (Variables|/Game/ThirdPerson/Blueprints/BP_ThirdPersonGameMode.BP_ThirdPersonGameMode_C|GetIsPileInDrone (stale EventBeginPlay _asbp_third_person_game_mode))
      (Rendering|SetVisibility (Variables|Default|GetPointLightComponent) true false)
      (if (> (Variables|/Script/Engine.LightComponentBase|GetIntensity (Variables|Default|GetPointLightComponent)) 0.0)
        _
        (else
          (Variables|Default|SetIsLightMax false)))
      (if (Variables|Default|GetIsLightMax)
        (Rendering|Components|Light|SetIntensity (Variables|Default|GetPointLightComponent) (- (Variables|/Script/Engine.LightComponentBase|GetIntensity (Variables|Default|GetPointLightComponent)) (* DeltaSeconds 3e+03)))
        (elif (> (Variables|/Script/Engine.LightComponentBase|GetIntensity (Variables|Default|GetPointLightComponent)) 2e+03)
          (Variables|Default|SetIsLightMax true)
          (Default|CallLightMax)
          (else
            (Rendering|Components|Light|SetIntensity (Variables|Default|GetPointLightComponent) (+ (Variables|/Script/Engine.LightComponentBase|GetIntensity (Variables|Default|GetPointLightComponent)) (* DeltaSeconds 3e+03)))))))))

(event EventBeginPlay
  ;[0.15 0.15 0.15 0.5] BlinkerTrackEmergency
  (bind _asbp_third_person_game_mode (Utilities|Casting|CastToBP_ThirdPersonGameMode (Game|GetGameMode)))
  (EventDispatchers|BindEventtoLightMax (delegate Custom|Sound)))

(fn ConstructionScript)