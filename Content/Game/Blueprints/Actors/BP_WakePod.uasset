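; BP_WakePod is an actor for the wake-up pod, animating its lift, opening and closing, including for the main menu to level 1 transition.
; LiftPod swaps a material on the Load component to M_Vitre, eases the pod mesh to a tilted pose and plays a series of effects, one slightly delayed.
; OpenPod and CloseMovement rotate Load between open and closed poses using timed MoveComponentTo calls.
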(event Custom|CloseMovement
  ;[0.15 0.15 0.15 0.5] Closing pod animation
  (Components|MoveComponentTo (Variables|Default|Getload) "28.644460,-3.667849,74.113936" "0.000000,180.000004,180.000000" false false 3.0 false))

(event Custom|OpenPod
  ;[0.15 0.15 0.15 0.5] Opening pod animation
  (Components|MoveComponentTo (Variables|Default|Getload) "28.644460,-3.667849,74.113936" "0.000000,-180.000004,280.000000" true false 3.0 false))

(event Custom|LiftPod
  ;[0.15 0.15 0.15 0.5] Lift the pod animation (usefull in mainmenu/lvl1 transition)
  (Rendering|Material|SetMaterial (Variables|Default|Getload) 3 "/Game/Game/Materials/M_Vitre.M_Vitre")
  (Audio|Components|Audio|Play (Variables|Default|GetPodLift) 0.0)
  (Components|MoveComponentTo (Variables|Default|GetStaticMeshComponent) "82.489637,90.440368,76.137171" "0.000000,-180.000000,40.000000" true true 4.0 false)
  (Audio|Components|Audio|Play (Variables|Default|GetClong) 0.0)
  (Audio|Components|Audio|Play (Variables|Default|GetUnfreeze) 0.0)
  (Utilities|FlowControl|Delay 0.4)
  (Audio|Components|Audio|Play (Variables|Default|GetPshhh) 0.0))

(fn ConstructionScript
  (|CallParentFunction))