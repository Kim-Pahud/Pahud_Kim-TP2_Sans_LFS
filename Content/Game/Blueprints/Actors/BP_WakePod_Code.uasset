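; Wake pod variant that, once opened, lets the player view a code card widget by interacting nearby.
; The Open event swaps a material on the Load component to M_Vitre and animates it to its open position.
; A child-actor enter zone tracks player presence and toggles the PressF prompt, shown only if the pod is open on entry.
; IA_Interact then shows the cursor, toggles camera input and displays WBP_CodeCard.
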(event Custom|SetOpen
  ;[0.15 0.15 0.15 0.5] Open pod animation (just the code pod (usefull for lvl2))
  (Variables|Default|SetIsOpen? true)
  (Rendering|Material|SetMaterial (Variables|Default|Getload) 3 "/Game/Game/Materials/M_Vitre.M_Vitre")
  (Components|MoveComponentTo (Variables|Default|Getload) "28.644460,-3.667849,74.113936" "0.000000,-180.000004,280.000000" false false 3.0 false))

(event Custom|OnPlayerEnter
  (params (Object :type Actor%20Object%20Reference))
  ;[0.15 0.15 0.15 0.5] Check if player is in range to interact with the code card
  (if (Variables|Default|GetIsOpen?)
    (Rendering|SetVisibility (Variables|Default|GetPress%28F%29) true false)
    (Variables|Default|SetIsPlayerIn? true)))

(event Custom|OnPlayerExit
  (params (Object :type Actor%20Object%20Reference))
  ;[0.15 0.15 0.15 0.5] Check if player is in range to interact with the code card
  (Rendering|SetVisibility (Variables|Default|GetPress%28F%29) false false)
  (Variables|Default|SetIsPlayerIn? false))

(event Input|EnhancedActionEvents|EnhancedInputActionIA_Interact
  (params (ActionValue :type Boolean) (ElapsedSeconds :type Float%20%28double-precision%29) (TriggeredSeconds :type Float%20%28double-precision%29) (InputAction :type Input%20Action%20Object%20Reference :default "/Game/Game/Systeme/Character/CustomInputs/IA_Interact.IA_Interact"))
  (bind _widget (Variables|Default|GetWidget))
  ;[0.15 0.15 0.15 0.5] Show code card widget When player press f
  (if (Variables|Default|GetIsOpen?)
    (if (Variables|Default|GetIsPlayerIn?)
      (Variables|/Script/Engine.PlayerController|SetbShowMouseCursor (Game|GetPlayerController 0) true)
      (Default|Activate/DesactivateCamInput (Variables|Default|GetAs%20BP%20Third%20Person%20Player%20Controller) _widget)
      (UserInterface|Viewport|AddtoViewport _widget 0))))

(event EventBeginPlay
  ;[0.15 0.15 0.15 0.5] Set all var and bind all event and custom inputs + create widdgets needed
  (|CallParentFunction)
  (EventDispatchers|BindEventtoOpen (delegate Custom|SetOpen))
  (bind _asbp_enter_zone_player (Utilities|Casting|CastToBP_EnterZone_Player (Variables|/Script/Engine.ChildActorComponent|GetChildActor (Variables|Default|GetCode_PickUp_Zone))))
  (EventDispatchers|BindEventtoOnPlayerEnter _asbp_enter_zone_player (EventDispatchers|CreateEvent :!event Custom|OnPlayerEnter))
  (EventDispatchers|BindEventtoOnPlayerExit _asbp_enter_zone_player (EventDispatchers|CreateEvent :!event Custom|OnPlayerExit))
  (bind _asbp_third_person_player_controller (Utilities|Casting|CastToBP_ThirdPersonPlayerController (Game|GetPlayerController 0)))
  (Variables|Default|SetAs%20BP%20Third%20Person%20Player%20Controller _asbp_third_person_player_controller)
  (bind _returnvalue (UserInterface|CreateWidget "/Game/Game/UI/Actor_UI/WBP_CodeCard.WBP_CodeCard_C"))
  (Variables|Default|SetWidget _returnvalue)
  (Input|EnableInput (Game|GetPlayerController 0))
  (Rendering|SetVisibility (Variables|Default|GetPress%28F%29) false false))

(event Collision|EventActorBeginOverlap
  (params (OtherActor :type Actor%20Object%20Reference))
  (|CallParentFunction OtherActor) ; Ce nœud est désactivé et ne sera pas appelé.\nFaites glisser les broches pour générer des fonctionnalités.
)

(event EventTick
  (params (DeltaSeconds :type Float%20%28single-precision%29))
  (|CallParentFunction DeltaSeconds) ; Ce nœud est désactivé et ne sera pas appelé.\nFaites glisser les broches pour générer des fonctionnalités.
)

(fn ConstructionScript
  (|CallParentFunction))