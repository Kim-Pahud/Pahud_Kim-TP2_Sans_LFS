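; BP_EmergencyDoorLight is an emergency door light that blinks once the fuse box is activated and turns green when Door 2 opens.
; It caches BP_ThirdPersonGameMode on BeginPlay and polls its door and fuse box flags every Tick.
; While blinking, it makes the point light visible and ramps intensity up and down with DeltaSeconds, using IsLightMax to flip direction.
; An open door takes priority, setting the color and halting the ramp.
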(event EventTick
  (params (DeltaSeconds :type Float%20%28single-precision%29))
  ;[0.15 0.15 0.15 0.5] BlinkerDoorEmergency
  (if (Variables|/Game/ThirdPerson/Blueprints/BP_ThirdPersonGameMode.BP_ThirdPersonGameMode_C|GetIsDoor2Open (stale EventBeginPlay _asbp_third_person_game_mode))
    ;[0.15 0.15 0.15 0.5] Change BlinkerDoor Color
    (Rendering|Components|Light|SetLightColor (Variables|Default|GetPointLightComponent) (Utilities|Struct|MakeLinearColor 0.122 1.0 0.074 0.0) true)
    (elif (Variables|/Game/ThirdPerson/Blueprints/BP_ThirdPersonGameMode.BP_ThirdPersonGameMode_C|GetIsFuseBoxActivated (stale EventBeginPlay _asbp_third_person_game_mode))
      (Rendering|SetVisibility (Variables|Default|GetPointLightComponent) true false)
      (if (> (Variables|/Script/Engine.LightComponentBase|GetIntensity (Variables|Default|GetPointLightComponent)) 0.0)
        _
        (else
          (Variables|Default|SetIsLightMax false)))
      (if (Variables|Default|GetIsLightMax)
        (Rendering|Components|Light|SetIntensity (Variables|Default|GetPointLightComponent) (- (Variables|/Script/Engine.LightComponentBase|GetIntensity (Variables|Default|GetPointLightComponent)) (* DeltaSeconds 1.5e+03)))
        (elif (> (Variables|/Script/Engine.LightComponentBase|GetIntensity (Variables|Default|GetPointLightComponent)) 2e+03)
          (Variables|Default|SetIsLightMax true)
          (else
            (Rendering|Components|Light|SetIntensity (Variables|Default|GetPointLightComponent) (+ (Variables|/Script/Engine.LightComponentBase|GetIntensity (Variables|Default|GetPointLightComponent)) (* DeltaSeconds 1.5e+03)))))))))

(event EventBeginPlay
  ;[0.15 0.15 0.15 0.5] BlinkerDoorEmergency
  (bind _asbp_third_person_game_mode (Utilities|Casting|CastToBP_ThirdPersonGameMode (Game|GetGameMode))))

(fn ConstructionScript)