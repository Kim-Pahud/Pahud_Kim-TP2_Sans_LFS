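; BP_FlightPlans is an interactable flight plan actor that signals objective completion when the player takes it.
; A BP_EnterZone_Player child actor reports player enter and exit, toggling the in-range flag and the Press F prompt.
; Tick blinks the FlightPlan component through a DoOnce that resets after a delay until the plan is taken.
; IA_Interact in range marks it taken, hides both components and calls PlayerHasPlan.
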(event Custom|On%20Player%20Enter
  (params (Object :type Actor%20Object%20Reference))
  ;[0.15 0.15 0.15 0.5] Set interaction range var and show interaction key
  (Variables|Default|SetIsPlayerIn? true)
  (Rendering|SetVisibility (Variables|Default|GetPress%20%28F%29) true false))

(event Custom|On%20Player%20Exit
  (params (Object :type Actor%20Object%20Reference))
  ;[0.15 0.15 0.15 0.5] Set interaction range var and show interaction key
  (Variables|Default|SetIsPlayerIn? false)
  (Rendering|SetVisibility (Variables|Default|GetPress%20%28F%29) false false))

(event Input|EnhancedActionEvents|EnhancedInputActionIA_Interact
  (params (ActionValue :type Boolean) (ElapsedSeconds :type Float%20%28double-precision%29) (TriggeredSeconds :type Float%20%28double-precision%29) (InputAction :type Input%20Action%20Object%20Reference :default "/Game/Game/Systeme/Character/CustomInputs/IA_Interact.IA_Interact"))
  ;[0.15 0.15 0.15 0.5] Send a cue for objective completion when player interact
  (if (Variables|Default|GetIsPlayerIn?)
    (Variables|Default|SetPlanTaken? true)
    (Rendering|SetVisibility (Variables|Default|GetPress%20%28F%29) false false)
    (Rendering|SetVisibility (Variables|Default|GetFlight%20Plan) false false)
    (Default|CallPlayerHasPlan)))

(event EventTick
  (params (DeltaSeconds :type Float%20%28single-precision%29))
  ;[0.15 0.15 0.15 0.5] Make the text blink
  (Utilities|FlowControl|DoOnce false :!label _label
    (:Completed
      (if (Variables|Default|GetIsMessageVisible?)
        (Rendering|SetVisibility (Variables|Default|GetFlight%20Plan) false false)
        (Variables|Default|SetIsMessageVisible? false)
        (else
          (Rendering|SetVisibility (Variables|Default|GetFlight%20Plan) true false)
          (Variables|Default|SetIsMessageVisible? true)))
      (Utilities|FlowControl|Delay 1.0)
      (if (not (Variables|Default|GetPlanTaken?))
        (goto _label Reset)))))

(event EventBeginPlay
  ;[0.15 0.15 0.15 0.5] Set all var, bind all event and inputs needed
  (bind _asbp_enter_zone_player (Utilities|Casting|CastToBP_EnterZone_Player (Variables|/Script/Engine.ChildActorComponent|GetChildActor (Variables|Default|GetInteraction%20Zone))))
  (bind _output_get (Variables|Default|SetAs%20BP%20Enter%20Zone%20Player _asbp_enter_zone_player))
  (EventDispatchers|BindEventtoOnPlayerEnter _output_get (EventDispatchers|CreateEvent :!event Custom|On%20Player%20Enter))
  (EventDispatchers|BindEventtoOnPlayerExit _output_get (EventDispatchers|CreateEvent :!event Custom|On%20Player%20Exit))
  (Input|EnableInput (Game|GetPlayerController 0)))

(fn ConstructionScript)