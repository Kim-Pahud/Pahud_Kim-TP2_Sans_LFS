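; Corridor-end door actor that can open or be destroyed on command, with alien banging sounds playing at it.
; Opening plays DoorOpening, eases the CorridorEnd component to a new transform and stops further banging, while destroying removes that component.
; Tick drives a DoOnce loop that plays random SonTab sounds at DoorDestroyed, spaced by random delays or a shorter fixed one when IsItLastMin is set.
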(event Custom|DoorOpen
  ;[0.15 0.15 0.15 0.5] Door opening animation
  (Audio|Components|Audio|Play (Variables|Default|GetDoorOpening) 0.0)
  (Components|MoveComponentTo (Variables|Default|Getcorridor_end) "0.500000,-5.000000,156.000000" "0.000000,180.000000,0.000000" true false 0.6 false)
  (Variables|Default|SetShouldPlay? false))

(event Custom|DestroyDoor
  ;[0.15 0.15 0.15 0.5] Destroy door on command
  (Components|DestroyComponent (Variables|Default|Getcorridor_end)))

(event Custom|DelayBetween
  ;[0.15 0.15 0.15 0.5] Alien Banging Sound loop
  (if (Variables|Default|GetIsItLastMin?)
    (Utilities|FlowControl|Delay 1.5)
    (Utilities|FlowControl|DoOnce false) ; enters at Reset
    (else
      (Utilities|FlowControl|Delay (Math|Random|RandomFloatinRange 3.0 5.0))
      (Utilities|FlowControl|DoOnce false) ; enters at Reset
    )))

(event EventTick
  (params (DeltaSeconds :type Float%20%28single-precision%29))
  ;[0.15 0.15 0.15 0.5] Alien Banging Sound loop
  (Utilities|FlowControl|DoOnce false
    (:Completed
      (if (Variables|Default|GetShouldPlay?)
        (bind _returnvalue (Audio|SpawnSoundatLocation (.OutItem (Utilities|Array|Random (Variables|Default|GetSonTab))) (Transformation|GetWorldLocation (Variables|Default|GetDoorDestroyed)) "0, 0, 0" 3.0 0.7 0.0 "/Game/Game/Audio/SFX/ATT_DoorPuch.ATT_DoorPuch" 0))
        (Audio|Components|Audio|Play _returnvalue 0.0))
      (CallFunction|DelayBetween))))

(fn ConstructionScript)