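; BP_PodZone is a trigger zone that cues the player for the final interaction at the pod.
; It caches BP_ThirdPersonGameMode on BeginPlay and reads its LightCheck flag on each overlap.
; When an actor tagged Player enters or leaves while that flag is true, it calls PlayerIn or PlayerOut to signal the change.
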(event Collision|EventActorBeginOverlap
  (params (OtherActor :type Actor%20Object%20Reference))
  ;[0.15 0.15 0.15 0.5] Cue Of Player For Final Interaction
  (if (Actor|ActorHasTag OtherActor "Player")
    (if (Variables|/Game/ThirdPerson/Blueprints/BP_ThirdPersonGameMode.BP_ThirdPersonGameMode_C|GetLightCheck (stale EventBeginPlay _output_get))
      (Default|CallPlayerin))))

(event Collision|EventActorEndOverlap
  (params (OtherActor :type Actor%20Object%20Reference))
  ;[0.15 0.15 0.15 0.5] Cue Of Player For Final Interaction
  (if (Actor|ActorHasTag OtherActor "Player")
    (if (Variables|/Game/ThirdPerson/Blueprints/BP_ThirdPersonGameMode.BP_ThirdPersonGameMode_C|GetLightCheck (stale EventBeginPlay _output_get))
      (Default|CallPlayerOut))))

(event EventBeginPlay
  ;[0.15 0.15 0.15 0.5] Cue Of Player For Final Interaction
  (bind _asbp_third_person_game_mode (Utilities|Casting|CastToBP_ThirdPersonGameMode (Game|GetGameMode)))
  (bind _output_get (Variables|Default|SetAs%20BP%20Third%20Person%20Game%20Mode _asbp_third_person_game_mode)))

(fn ConstructionScript)