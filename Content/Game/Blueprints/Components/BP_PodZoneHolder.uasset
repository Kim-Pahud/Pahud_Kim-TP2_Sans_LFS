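; BP_PodZoneHolder is an actor that shows a "Press F" prompt for the final interaction while the player is inside its pod zone.
; On BeginPlay it casts its PodZone child actor to BP_PodZone and binds to that zone's player-in and player-out events.
; Those events toggle the PressF component's visibility and the PlayerInBox flag; the F key input itself is not handled here.
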(event Custom|PlayerIn
  ;[0.15 0.15 0.15 0.5] Visibility Of Press F For Final Interaction
  (Rendering|SetVisibility (Variables|Default|GetPress%28f%29) true false)
  (Variables|Default|SetPlayerInBox true))

(event Custom|PlayerOut
  ;[0.15 0.15 0.15 0.5] Visibility Of Press F For Final Interaction
  (Rendering|SetVisibility (Variables|Default|GetPress%28f%29) false false)
  (Variables|Default|SetPlayerInBox false))

(event EventBeginPlay
  ;[0.15 0.15 0.15 0.5] Visibility Of Press F For Final Interaction
  (bind _asbp_pod_zone (Utilities|Casting|CastToBP_PodZone (Variables|/Script/Engine.ChildActorComponent|GetChildActor (Variables|Default|GetPodZone))))
  (bind _output_get (Variables|Default|SetAs%20BP%20Pod%20Zone _asbp_pod_zone))
  (EventDispatchers|BindEventtoPlayerin _output_get (delegate Custom|PlayerIn))
  (EventDispatchers|BindEventtoPlayerOut _output_get (delegate Custom|PlayerOut)))

(fn ConstructionScript)