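; BP_BlinkSpotLight is a spotlight that flickers randomly with sound while it is visible.
; BeginPlay hides the light, and nothing in this file shows it again.
; While it is visible, Tick uses a short Delay to throttle calls to Blink.
; Blink compares a random roll to LightRate, setting either minimum intensity with the SBlinkSpotLight sound or full intensity.
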(event EventTick
  (params (DeltaSeconds :type Float%20%28single-precision%29))
  ;[0.15 0.15 0.15 0.5] Set The Delay Between 2 Blink
  (if (Rendering|IsVisible (Variables|Default|GetSpotLightComponent))
    (Utilities|FlowControl|Delay 0.2)
    (CallFunction|Blink (Variables|Default|GetMinIntensity) (Variables|Default|GetMaxIntensity))))

(event EventBeginPlay
  ;[0.15 0.15 0.15 0.5] Set The Delay Between 2 Blink
  (Rendering|SetVisibility (Variables|Default|GetSpotLightComponent) false false))

(fn ConstructionScript)

(fn Blink
  (params (MinIntensity :type Float%20%28double-precision%29) (FullIntensity :type Float%20%28double-precision%29))
  ;[0.15 0.15 0.15 0.5] Make The SpotLight Blink
  (if (> (Math|Random|RandomFloatinRange 0.0 1.0) (Variables|Default|GetLightRate))
    (Rendering|Components|Light|SetIntensity (Variables|Default|GetSpotLightComponent) MinIntensity)
    (Audio|Components|Audio|Play (Variables|Default|GetS_BlinkSpotLight) 0.0)
    (else
      (Rendering|Components|Light|SetIntensity (Variables|Default|GetSpotLightComponent) FullIntensity))))