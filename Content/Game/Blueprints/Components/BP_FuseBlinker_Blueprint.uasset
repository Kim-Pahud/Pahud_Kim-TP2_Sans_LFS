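; BP_FuseBlinker is a Blueprint that makes a point light blink and change color, apparently as a fuse indicator.
; Blinker ramps the light intensity up and down by scaled delta time, using the IsLightMax flag to reverse at the given maximum and at zero.
; ColorChanger sets the light color from RGBA inputs.
; No event in this graph calls either function, so timing and color come from outside callers.
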(fn ConstructionScript)

(fn Blinker
  (params (DeltaSec :type Float%20%28double-precision%29) (MaxIntensity :type Float%20%28double-precision%29) (DeltaMultiplier :type Float%20%28double-precision%29))
  ;[0.15 0.15 0.15 0.5] Make a Light Blink
  (if (> (Variables|/Script/Engine.LightComponentBase|GetIntensity (Variables|Default|GetPointLightComponent)) 0.0)
    _
    (else
      (Variables|Default|SetIsLightMax false)))
  (if (Variables|Default|GetIsLightMax)
    (Rendering|Components|Light|SetIntensity (Variables|Default|GetPointLightComponent) (- (Variables|/Script/Engine.LightComponentBase|GetIntensity (Variables|Default|GetPointLightComponent)) (* DeltaSec DeltaMultiplier)))
    (elif (> (Variables|/Script/Engine.LightComponentBase|GetIntensity (Variables|Default|GetPointLightComponent)) MaxIntensity)
      (Variables|Default|SetIsLightMax true)
      (else
        (Rendering|Components|Light|SetIntensity (Variables|Default|GetPointLightComponent) (+ (Variables|/Script/Engine.LightComponentBase|GetIntensity (Variables|Default|GetPointLightComponent)) (* DeltaSec DeltaMultiplier)))))))

(fn ColorChanger
  (params (R :type Float%20%28double-precision%29) (G :type Float%20%28double-precision%29) (B :type Float%20%28double-precision%29) (A :type Float%20%28double-precision%29))
  ;[0.15 0.15 0.15 0.5] Change Blinker Color
  (Rendering|Components|Light|SetLightColor (Variables|Default|GetPointLightComponent) (Utilities|Struct|MakeLinearColor R G B A) true))