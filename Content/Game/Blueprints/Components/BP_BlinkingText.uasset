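; BP_BlinkingText is a Blueprint that makes its TextRender blink by alternately showing and hiding it.
; Tick drives a DoOnce gate, which flips the text's visibility and the IsVisible flag, then waits BlinkRate seconds before resetting.
; The gate and Delay turn the per-frame Tick into a repeating blink cycle without a timer.
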(event EventTick
  (params (DeltaSeconds :type Float%20%28single-precision%29))
  (Utilities|FlowControl|DoOnce false :!label _label
    (:Completed
      (if (Variables|Default|GetIsVisible)
        (Rendering|SetVisibility (Variables|Default|GetTextRender) false false)
        (Variables|Default|SetIsVisible false)
        (Utilities|FlowControl|Delay (Variables|Default|GetBlinkRate))
        (goto _label Reset)
        (else
          (Rendering|SetVisibility (Variables|Default|GetTextRender) true false)
          (Variables|Default|SetIsVisible true)
          (Utilities|FlowControl|Delay (Variables|Default|GetBlinkRate))
          (goto _label Reset))))))

(fn ConstructionScript)