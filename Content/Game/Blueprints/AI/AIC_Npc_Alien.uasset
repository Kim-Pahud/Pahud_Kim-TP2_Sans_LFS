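; AI controller for alien NPCs that adds a toggleable debug view of the NPC's vision ranges.
; On BeginPlay it binds to the player controller's debug toggle, which flip-flops between starting and pausing a fast looping timer.
; Each tick of that timer reads the Vision settings and draws the secondary cone's two edges and the proximity radius circle from the pawn's eye viewpoint.
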(event Custom|Toggle%20Debugg%20Vision%20Cone
  (Utilities|FlowControl|FlipFlop
    (:A
      (bind _returnvalue (Utilities|Time|SetTimerbyFunctionName 0 "Draw Debug Vision Cones" 0.01 true true))
      (Variables|Default|SetTimer _returnvalue))
    (:B
      (Utilities|Time|PauseTimerbyHandle (Variables|Default|GetTimer)))))

(event EventBeginPlay
  (bind _asbp_third_person_player_controller (Utilities|Casting|CastToBP_ThirdPersonPlayerController (Game|GetPlayerController 0)))
  (Utilities|IsValid _asbp_third_person_player_controller
    (:Is%20Valid
      (EventDispatchers|BindEventtoToggleDebugVisionCone _asbp_third_person_player_controller (EventDispatchers|CreateEvent :!event Custom|Toggle%20Debugg%20Vision%20Cone)))))

(fn ConstructionScript)

(fn DrawDebugVisionCones
  (bind _returnvalue (Pawn|GetControlledPawn))
  (bind _returnvalue_2 (Pawn|GetControlledPawn))
  (bind (_outlocation _outrotation) (Actor|GetActorEyesViewPoint _returnvalue_2))
  (bind (_outlocation_2 _outrotation_2) (Actor|GetActorEyesViewPoint _returnvalue))
  (Rendering|Debug|DrawDebugLine _outlocation_2 (+ (* (Math|Vector|GetForwardVector (Math|Rotator|CombineRotators _outrotation_2 (Math|Rotator|MakeRotator 0.0 0.0 (.SecondaryVisionConeAngle (Utilities|Struct|BreakF_SecondaryVisionConeInfos (Variables|Default|GetVision)))))) (Utilities|Struct|BreakF_SecondaryVisionConeInfos (Variables|Default|GetVision))) _outlocation_2) "(R=1.000000,G=0.000000,B=0.000000,A=1.000000)" 0.0 0.0)
  (Rendering|Debug|DrawDebugLine _outlocation (+ (* (Math|Vector|GetForwardVector (Math|Rotator|CombineRotators _outrotation (Math|Rotator|MakeRotator 0.0 0.0 (* (Utilities|Struct|BreakF_SecondaryVisionConeInfos (Variables|Default|GetVision)) -1.0)))) (Utilities|Struct|BreakF_SecondaryVisionConeInfos (Variables|Default|GetVision))) _outlocation) "(R=1.000000,G=0.000000,B=0.000000,A=1.000000)" 0.0 0.0)
  (Rendering|Debug|DrawDebugCircle (.OutLocation (Actor|GetActorEyesViewPoint (Pawn|GetControlledPawn))) (Utilities|Struct|BreakF_SecondaryVisionConeInfos (Variables|Default|GetVision)) 30 "(R=0.068420,G=1.000000,B=0.046811,A=1.000000)" 0.0 0.0 "1.000000,0.000000,0.000000" "0.000000,1.000000,0.000000"))