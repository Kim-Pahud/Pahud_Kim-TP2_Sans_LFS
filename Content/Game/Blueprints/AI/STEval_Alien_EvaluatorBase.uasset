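; Base StateTree evaluator for the Alien AI that hooks into the perception components on the alien's AI controller.
; On tree start it binds to target perception updates from the direct, secondary and proximity perception components, plus forgotten-target events from the direct one.
; On tree stop it unbinds them all.
; The handler events are empty here, leaving the actual response to stimuli to derived evaluators.
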(event Custom|Event%20To%20On%20Target%20Perception%20Updated
  (params (Actor :type Actor%20Object%20Reference) (Stimulus :type AI%20Stimulus%20Structure)))

(event Custom|Event%20On%20Target%20Perception%20Forgotten
  (params (Actor :type Actor%20Object%20Reference)))

(event Custom|Secondary%20On%20Target%20Perception%20Updated
  (params (Actor :type Actor%20Object%20Reference) (Stimulus :type AI%20Stimulus%20Structure)))

(event Custom|Proximity%20On%20Target%20Perception%20Updated
  (params (Actor :type Actor%20Object%20Reference) (Stimulus :type AI%20Stimulus%20Structure)))

(event EventTreeStart
  (EventDispatchers|BindEventtoOnTargetPerceptionUpdated (Variables|/Game/Game/Blueprints/AI/AIC_Npc_Alien.AIC_Npc_Alien_C|GetAIPerceptionDirect (Variables|Contexte|GetAlien%20AI%20Controller%20Ref)) (EventDispatchers|CreateEvent :!event Custom|Event%20To%20On%20Target%20Perception%20Updated))
  (EventDispatchers|BindEventtoOnTargetPerceptionForgotten (Variables|/Game/Game/Blueprints/AI/AIC_Npc_Alien.AIC_Npc_Alien_C|GetAIPerceptionDirect (Variables|Contexte|GetAlien%20AI%20Controller%20Ref)) (EventDispatchers|CreateEvent :!event Custom|Event%20On%20Target%20Perception%20Forgotten))
  (EventDispatchers|BindEventtoOnTargetPerceptionUpdated (Variables|/Game/Game/Blueprints/AI/AIC_Npc_Alien.AIC_Npc_Alien_C|GetAIPerceptionSecondary (Variables|Contexte|GetAlien%20AI%20Controller%20Ref)) (EventDispatchers|CreateEvent :!event Custom|Secondary%20On%20Target%20Perception%20Updated))
  (EventDispatchers|BindEventtoOnTargetPerceptionUpdated (Variables|/Game/Game/Blueprints/AI/AIC_Npc_Alien.AIC_Npc_Alien_C|GetAIPerceptionProximity (Variables|Contexte|GetAlien%20AI%20Controller%20Ref)) (EventDispatchers|CreateEvent :!event Custom|Proximity%20On%20Target%20Perception%20Updated)))

(event EventTreeStop
  (EventDispatchers|UnbindEventfromOnTargetPerceptionUpdated (Variables|/Game/Game/Blueprints/AI/AIC_Npc_Alien.AIC_Npc_Alien_C|GetAIPerceptionDirect (Variables|Contexte|GetAlien%20AI%20Controller%20Ref)) (EventDispatchers|CreateEvent :!event Custom|Event%20To%20On%20Target%20Perception%20Updated))
  (EventDispatchers|UnbindEventfromOnTargetPerceptionForgotten (Variables|/Game/Game/Blueprints/AI/AIC_Npc_Alien.AIC_Npc_Alien_C|GetAIPerceptionDirect (Variables|Contexte|GetAlien%20AI%20Controller%20Ref)) (EventDispatchers|CreateEvent :!event Custom|Event%20On%20Target%20Perception%20Forgotten))
  (EventDispatchers|UnbindEventfromOnTargetPerceptionUpdated (Variables|/Game/Game/Blueprints/AI/AIC_Npc_Alien.AIC_Npc_Alien_C|GetAIPerceptionSecondary (Variables|Contexte|GetAlien%20AI%20Controller%20Ref)) (EventDispatchers|CreateEvent :!event Custom|Secondary%20On%20Target%20Perception%20Updated))
  (EventDispatchers|UnbindEventfromOnTargetPerceptionUpdated (Variables|/Game/Game/Blueprints/AI/AIC_Npc_Alien.AIC_Npc_Alien_C|GetAIPerceptionProximity (Variables|Contexte|GetAlien%20AI%20Controller%20Ref)) (EventDispatchers|CreateEvent :!event Custom|Proximity%20On%20Target%20Perception%20Updated)))