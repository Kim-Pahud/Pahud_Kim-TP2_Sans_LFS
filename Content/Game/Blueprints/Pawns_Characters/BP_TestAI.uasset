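; BP_TestAI is a test AI Blueprint that accumulates a Patience value over time, scaled by the current level.
; On BeginPlay it reads the live level name from BP_MyGameInstance and sets a higher LevelMultiplier for level1 than for other levels.
; Each Tick adds delta time times that multiplier to Patience, which nothing in this Blueprint reads or acts on.
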(event EventBeginPlay
  (bind _asbp_my_game_instance (Utilities|Casting|CastToBP_MyGameInstance (Game|GetGameInstance)))
  (bind _output_get (Variables|Default|SetAs%20BP%20My%20Game%20Instance _asbp_my_game_instance))
  (if (Utilities|Enum|Equal(Enum) (Variables|/Game/Game/Systeme/BP_MyGameInstance.BP_MyGameInstance_C|GetLiveLevelName _output_get) "level1")
    (Variables|Default|SetLevelMultiplier 2.0)
    (else
      (Variables|Default|SetLevelMultiplier 1.0))))

(event EventTick
  (params (DeltaSeconds :type Float%20%28single-precision%29))
  (Variables|Default|SetPatience (+ (* DeltaSeconds (Variables|Default|GetLevelMultiplier)) (Variables|Default|GetPatience))))

(fn ConstructionScript)